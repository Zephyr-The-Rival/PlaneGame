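; AC_Tank is an actor component that tracks a tank's fill level as a normalized value, starting empty at BeginPlay.
; FillTank and ReduceTank add or subtract the absolute value of the given amount, clamping the level between empty and full.
; A RepNotify on FillLevel broadcasts the empty, full or changed event dispatcher, passing the current level only for intermediate values.
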(event `self.ReceiveBeginPlay`
  (set `self.FillLevel` 0.0))

(fn `FillTank`
  (params (FillAmount :type "Float (double-precision)"))
  (bind _returnvalue (+ (`self.FillLevel`) (`KismetMathLibrary.Abs` FillAmount)))
  (if (< (`self.FillLevel`) 1.0)
    (if (> _returnvalue 1.0)
      (set `self.FillLevel` 1.0)
      (else
        (set `self.FillLevel` _returnvalue)))))

(fn `OnRep_FillLevel`
  (if (== (`self.FillLevel`) 0.0)
    (`self.OnTankEmpty`)
    (elif (== (`self.FillLevel`) 1.0)
      (`self.OnTankFull`)
      (else
        (`self.OnTankChanged` (`self.FillLevel`))))))

(fn `ReduceTank`
  (params (`Reduce Amount` :type "Float (double-precision)"))
  (bind _returnvalue (- (`self.FillLevel`) (`KismetMathLibrary.Abs` `Reduce Amount`)))
  (if (> (`self.FillLevel`) 0.0)
    (if (< _returnvalue 0.0)
      (set `self.FillLevel` 0.0)
      (else
        (set `self.FillLevel` _returnvalue)))))