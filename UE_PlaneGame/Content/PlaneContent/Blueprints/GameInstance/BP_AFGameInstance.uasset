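; Game instance that handles online session hosting and invite-based joining through Advanced Sessions.
; CreateSession creates a named session and, on success, server-travels to TestMap as a listen server.
; It then immediately calls CheckForPlaneManager, which prints a red error unless exactly one BP_PlaneManager exists; the returned bool is unused.
; Accepted invites join the received session, with progress and results only printed as debug strings.
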(event `CreateSession`
  (params (SessionName :type String))
  (`CreateSessionCallbackProxyAdvanced.CreateAdvancedSession` (`|MakeArray` (`AdvancedSessionsLibrary.MakeLiteralSessionPropertyString` "SessionName" SessionName)) (`GameplayStatics.GetPlayerController` 0)
    (:`then`
      (`KismetSystemLibrary.PrintString` "Creating Session..."))
    (:`OnSuccess`
      (`AdvancedSessionsLibrary.ServerTravel` "/Game/PlaneContent/Maps/TestMap?listen" true)
      (`KismetSystemLibrary.PrintString` "BLUEPRINTS ON SUCCEED")
      (`self.CheckForPlaneManager`))
    (:`OnFailure`
      (`KismetSystemLibrary.PrintString` "Creating Advanced Session failed"))))

(event `self.OnSessionInviteAccepted`
  (params (LocalPlayerNum :type Integer) (PersonInvited :type "BPUniqueNetId Structure") (SessionToJoin :type "BlueprintSessionResult Structure (by ref)"))
  (`JoinSessionCallbackProxy.JoinSession` (`GameplayStatics.GetPlayerController` 0) SessionToJoin
    (:`then`
      (`KismetSystemLibrary.PrintString` "Join via invite"))
    (:`OnSuccess`
      (`KismetSystemLibrary.PrintString` "Join seession via invite  succeeded"))
    (:`OnFailure`
      (`KismetSystemLibrary.PrintString` "Join seession via invite  failed"))))

(fn `CheckForPlaneManager`
  (returns (`EverythingOkay?` :type Boolean))
  (bind _outactors (`GameplayStatics.GetAllActorsOfClass` "/Game/PlaneContent/Blueprints/Systems/Managers/BP_PlaneManager.BP_PlaneManager_C"))
  (if (`KismetArrayLibrary.Array_IsNotEmpty` _outactors)
    (if (== (`KismetArrayLibrary.Array_Length` _outactors) 1)
      (return true)
      (else
        (`KismetSystemLibrary.PrintString` "MORE THAN ONE \"PLANE MANAGER\" IN LEVEL!!!!" true true (struct :`R` 1.0 :`A` 1.0) 50.0)))
    (else
      (`KismetSystemLibrary.PrintString` "NO \"PLANE MANAGER\" IN LEVEL!!!!" true true (struct :`R` 1.0 :`A` 1.0) 50.0)))
  (return false))