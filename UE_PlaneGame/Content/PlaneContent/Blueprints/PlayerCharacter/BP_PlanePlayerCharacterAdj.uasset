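; Player character Blueprint for the plane game, with a child-actor hand and a physically animated "live ragdoll" body.
; On BeginPlay it registers itself as the hand's owner, then simulates the body through PhysicalAnimation, with physics disabled from the Arm bone down to keep it attached to the hand control.
; Key 1 cleans every stain actor in the level.
; An early full-body ragdoll function and a hand-range debug circle are left unconnected.
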(event `self.ReceiveBeginPlay`
  (bind _fullbody (`self.FullBody`))
  (bind _mesh (`self.Mesh`))
  (bind _physicalanimation (`self.PhysicalAnimation`))
  (`|ExecutionSequence`
    (:`then_0`
      (bind _asbp_player_hand (cast `/Game/PlaneContent/Blueprints/PlayerCharacter/BP_PlayerHand` (`ChildActorComponent.ChildActor` (`self.PlayerHandCA`))))
      (set `/Game/PlaneContent/Blueprints/PlayerCharacter/BP_PlayerHand.OwningPlayer` self _asbp_player_hand))
    (:`then_1`
      ;[0.1018 0 0.15 0.5] Live Ragdoll
      (`PhysicalAnimationComponent.SetSkeletalMeshComponent` _physicalanimation _mesh)
      (`PhysicalAnimationComponent.ApplyPhysicalAnimationSettingsBelow` _physicalanimation _fullbody (make `PhysicalAnimationData` true 1000.0 100.0 100.0 100.0 100.0 100.0) true)
      (`SkeletalMeshComponent.SetAllBodiesBelowSimulatePhysics` _mesh _fullbody true true)
      (`SkeletalMeshComponent.SetAllBodiesBelowPhysicsDisabled` _mesh (`self.Arm`) true true))))

(event `Key|One`
  (params (Key :type "Key Structure"))
  (:`Pressed`
    (bind _outactors (`GameplayStatics.GetAllActorsOfClass` "/Game/PlaneContent/Blueprints/MiniGame/BP_Stains.BP_Stains_C"))
    (for _array_element _outactors
      (`/Game/PlaneContent/Blueprints/MiniGame/BP_Stains.CleanStain` _array_element))))

(event `self.ReceiveTick`
  (params (DeltaSeconds :type "Float (single-precision)")))

(event `Key|^`
  (params (Key :type "Key Structure"))
  ;[0.1018 0 0.15 0.5] This was a start of the fullbody ragdoll
)

(event `MC_SetSpeechBubble_NeedEnum`
  (params (Need :type "/Game/PlaneContent/Blueprints/Systems/Passenger/Components/Needs/Enum_PassengerNeeds Enum" :default "NewEnumerator6")))

(fn `Start Ragdoll`
  (bind _mesh (`self.Mesh`))
  (`CharacterMovementComponent.SetMovementMode` (`self.CharacterMovement`) "MOVE_None" 0)
  (`PrimitiveComponent.SetCollisionEnabled` (`self.CapsuleComponent`) "NoCollision")
  (`PrimitiveComponent.SetCollisionObjectType` _mesh "ECC_PhysicsBody")
  (`PrimitiveComponent.SetCollisionEnabled` _mesh "QueryAndPhysics")
  (`SkeletalMeshComponent.SetAllBodiesBelowSimulatePhysics` _mesh "Pelvis" true true)
  (`SkeletalMeshComponent.SetAllBodiesBelowPhysicsBlendWeight` _mesh "Pelvis" 1.0 true true)
  (`KismetSystemLibrary.PrintString` "Ragdoll!"))

(fn `UserConstructionScript`)