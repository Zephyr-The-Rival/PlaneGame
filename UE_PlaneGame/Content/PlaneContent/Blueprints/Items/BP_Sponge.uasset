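; BP_Sponge is a cleaning tool that removes stains from BP_Stains actors.
; While active, it runs a complex multi-line visibility trace each Tick between its Start and End points.
; Stain hits are cached, and their collision UV positions the stain's DrawBrush call at the sponge's brush size.
; Reaching a movement threshold calls CleanStain on the cached stain, which clears on deactivation or a trace miss.
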(event `self.ActivateTool`
  (params (MovementVector :type "Vector Structure"))
  (set `self.bScanningActive` true))

(event `self.DeactivateTool`
  (set `self.bScanningActive` false)
  (set `self.StainsInstance` null))

(event `self.OnMovementThresholdReached`
  (bind _stainsinstance (`self.StainsInstance`))
  (if (`KismetSystemLibrary.IsValid` _stainsinstance)
    (`/Game/PlaneContent/Blueprints/MiniGame/Cleaning/BP_Stains.CleanStain` _stainsinstance)))

(event `self.ReceiveTick`
  (params (DeltaSeconds :type "Float (single-precision)"))
  (if (`self.bScanningActive`)
    (bind (_outhits _returnvalue) (`KismetSystemLibrary.LineTraceMulti` (`SceneComponent.K2_GetComponentLocation` (`self.Start`)) (`SceneComponent.K2_GetComponentLocation` (`self.End`)) "TraceTypeQuery1" true))
    (if _returnvalue
      (for _array_element _outhits
        (bind _asbp_stains (cast `/Game/PlaneContent/Blueprints/MiniGame/Cleaning/BP_Stains` (`.HitActor` (`GameplayStatics.BreakHitResult` _array_element))))
        (bind _output_get (set `self.StainsInstance` _asbp_stains))
        (bind (_uv _returnvalue_2) (`GameplayStatics.FindCollisionUV` _array_element))
        (if _returnvalue_2
          (`/Game/PlaneContent/Blueprints/MiniGame/Cleaning/BP_Stains.DrawBrush` _output_get (`self.BrushSize`) (`KismetMathLibrary.MakeVector2D` (`KismetMathLibrary.BreakVector2D` _uv) (`.Y` (`KismetMathLibrary.BreakVector2D` _uv))))))
      (else
        (set `self.StainsInstance` null)))))

(fn `UserConstructionScript`)