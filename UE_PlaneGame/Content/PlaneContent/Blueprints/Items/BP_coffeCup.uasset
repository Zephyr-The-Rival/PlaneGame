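; Coffee cup item that simulates spillage by lowering a liquid plane from full toward empty.
; Construction and BeginPlay set the plane to the full level.
; Each tick, four point-pair line traces run on a custom channel without ignoring the cup itself; each hit drains the level at a fixed rate scaled by delta time.
; Debug trace drawing and printed messages for hits and an empty cup remain active.
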(event `self.ReceiveBeginPlay`
  (`self.InitializeLiquidPlane`))

(event `self.ReceiveTick`
  (params (DeltaSeconds :type "Float (single-precision)"))
  (`|ExecutionSequence`
    (:`then_0`
      (`self.CheckAndHandleSpillage` (`SceneComponent.K2_GetComponentLocation` (`self.point1`)) (`SceneComponent.K2_GetComponentLocation` (`self.point1_1`)) DeltaSeconds))
    (:`then_1`
      (`self.CheckAndHandleSpillage` (`SceneComponent.K2_GetComponentLocation` (`self.point2`)) (`SceneComponent.K2_GetComponentLocation` (`self.point2_1`)) DeltaSeconds))
    (:`then_2`
      (`self.CheckAndHandleSpillage` (`SceneComponent.K2_GetComponentLocation` (`self.point3`)) (`SceneComponent.K2_GetComponentLocation` (`self.point3_1`)) DeltaSeconds))
    (:`then_3`
      (`self.CheckAndHandleSpillage` (`SceneComponent.K2_GetComponentLocation` (`self.point4`)) (`SceneComponent.K2_GetComponentLocation` (`self.point4_1`)) DeltaSeconds))))

(fn `CheckAndHandleSpillage`
  (params (Start :type "Vector Structure") (End :type "Vector Structure") (`delta time` :type "Float (double-precision)"))
  (locals (`Detect height` :type "Float (double-precision)" :default 55.0))
  (if (>= (`self.Current liquid level`) (`self.Empty liquid level`))
    (bind (_outhits _returnvalue) (`KismetSystemLibrary.LineTraceMulti` :`Start` Start :`End` End :`TraceChannel` "TraceTypeQuery3" :`DrawDebugType` "ForOneFrame" :`bIgnoreSelf` false))
    (if _returnvalue
      (`KismetSystemLibrary.PrintString` "Hello")
      (bind _output_get (set `self.Current liquid level` (- (`self.Current liquid level`) (* (`local.delta time`) 50.0))))
      (`SceneComponent.K2_SetRelativeLocation` (`self.LiquidPlane`) (`KismetMathLibrary.MakeVector` 0.0 0.0 _output_get) false false))
    (else
      (`KismetSystemLibrary.PrintString` "cup is empty" true true (struct :`G` 0.66 :`B` 1.0 :`A` 1.0) 2.0 "1"))))

(fn `InitializeLiquidPlane`
  (`SceneComponent.K2_SetRelativeLocation` (`self.LiquidPlane`) (`KismetMathLibrary.MakeVector` 0.0 0.0 (`self.Full liquid level`)) false false)
  (set `self.Current liquid level` (`self.Full liquid level`)))

(fn `UserConstructionScript`
  (`self.InitializeLiquidPlane`))