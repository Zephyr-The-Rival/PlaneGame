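; Actor component that makes its owner a smoke source, feeding a fixed smoke strength into nearby Actor_SmokeEmitters.
; It connects to the nearest emitters in range up to a cap, ignoring walls, and re-evaluates them on a timer after sufficient movement.
; A second timer redistributes strength by normalized inverse-square distance, replacing each emitter's recorded contribution.
; EndPlay withdraws all contributions; optional debug lines show connections and strengths.
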(event `self.ReceiveBeginPlay`
  (`|ExecutionSequence`
    (:`then_0`
      (`self.ConnectToSmokeEmitter`))
    (:`then_1`
      (`KismetSystemLibrary.K2_SetTimerDelegate` (`|CreateDelegate` :!event `UpdateEmitterDetection`) (`self.UpdateEmitterDetectionTick`) true))
    (:`then_2`
      (`KismetSystemLibrary.K2_SetTimerDelegate` (`|CreateDelegate` :!event `UpdateSmokeStrength`) (`self.UpdateSmokeStrengthTick`) true))
    (:`then_3`
      (set `self.LastPositionEmitterDetectionTick` (`Actor.K2_GetActorLocation` (`self.GetOwner`))))))

(event `self.ReceiveTick`
  (params (DeltaSeconds :type "Float (single-precision)"))
  (`|ExecutionSequence`
    (:`then_0`
      ; Debug
      (`self.DrawDebugLines`))))

(event `DrawDebugLines_Editor`
  ; Debug
  (`self.DrawDebugLines`))

(event `UpdateEmitterDetection`
  (if (`self.CheckForValidEmitterDetectionUpdate`)
    (`self.UpdateConnectedEmitter`)))

(event `UpdateSmokeStrength`
  (`self.UpdateSmokeValueInEmitter`))

(event `self.ReceiveEndPlay`
  (params (EndPlayReason :type "EEndPlayReason Enum" :default "Destroyed"))
  (for _array_element (`self.LastSmokeAmoutsStengthAddedToSmokeEmitter`)
    (bind (_smokeemitter _lastsmokestrength) (break `/Game/PlaneContent/Blueprints/Physics/Smoke/St_SmokeSource` _array_element))
    (`/Game/PlaneContent/Blueprints/Physics/Smoke/Actor_SmokeEmitter.DecreaseSmokeValue` _smokeemitter _lastsmokestrength)))

(fn `ConnectEmitter`
  (params (EmitterToConnect :type "/Game/PlaneContent/Blueprints/Physics/Smoke/Actor_SmokeEmitter Object Reference"))
  (bind _returnvalue (== (`KismetArrayLibrary.Array_Length` (`self.ConnectedSmokeEmitter`)) 1))
  (if (< (`KismetArrayLibrary.Array_Length` (`self.ConnectedSmokeEmitter`)) (`self.MaxEmitterConnectionCount`))
    (`KismetArrayLibrary.Array_Add` (`self.ConnectedSmokeEmitter`) EmitterToConnect)
    (bind _realsmokestrength (`self.GetRealSmokeStrength` EmitterToConnect))
    ; Strength is 0 when only one Emitter is connected
    (if _returnvalue
      (bind _returnvalue_2 (`KismetMathLibrary.SelectFloat` (`self.SmokeStrength`) _realsmokestrength _returnvalue))
      (`/Game/PlaneContent/Blueprints/Physics/Smoke/Actor_SmokeEmitter.IncreaseSmokeValue` EmitterToConnect _returnvalue_2))
    (`KismetArrayLibrary.Array_Add` (`self.LastSmokeAmoutsStengthAddedToSmokeEmitter`) (make `/Game/PlaneContent/Blueprints/Physics/Smoke/St_SmokeSource` EmitterToConnect _returnvalue_2))
    (`self.UpdateSmokeValueInEmitter`)
    (else
      (`KismetSystemLibrary.PrintString` (`KismetStringLibrary.Concat_StrStr` (`KismetSystemLibrary.GetDisplayName` (`self.GetOwner`)) ": " "Tried to connect more Emitters then allowed in Smoke Source Component") true true (struct :`G` 0.66 :`B` 1.0 :`A` 1.0) 8.0))))

(fn `ConnectToSmokeEmitter`
  (locals (Emitters :type "Array of /Game/PlaneContent/Blueprints/Physics/Smoke/Actor_SmokeEmitter Object Reference") (SearchIndex :type Integer) (ClosestDistance :type "Float (single-precision)" :default 0.0) (NearestEmitter :type "/Game/PlaneContent/Blueprints/Physics/Smoke/Actor_SmokeEmitter Object Reference"))
  ;[0.15 0.000781 0.000781 0.5] Would also check for emitter through walls / Raycast would fix this / Better would be just to consider emitters which are in the same room as the smoke source so no raycast or extra checks are necessary
  (bind _outactors (`GameplayStatics.GetAllActorsOfClass` "/Game/PlaneContent/Blueprints/Physics/Smoke/Actor_SmokeEmitter.Actor_SmokeEmitter_C")) ; Change to actors from room
  (bind _output_get (set `local.Emitters` _outactors))
  (if (>= (`KismetArrayLibrary.Array_Length` _output_get) (`self.MaxEmitterConnectionCount`))
    (set `local.SearchIndex` (`self.MaxEmitterConnectionCount`))
    (else
      (set `local.SearchIndex` (`KismetArrayLibrary.Array_Length` (`local.Emitters`)))))
  (for _ (range 1 (+ (`local.SearchIndex`) 1))
    (set `local.ClosestDistance` (`self.MaxEmitterConnectDistance`))
    (for _array_element (`local.Emitters`)
      ; Check if emitter is already connected
      (if (not (`KismetArrayLibrary.Array_Contains` (`self.ConnectedSmokeEmitter`) _array_element))
        ; Check if emitter is in range
        (if (`self.CheckIfEmitterIsInRange` _array_element)
          (bind _returnvalue (`Actor.GetDistanceTo` _array_element (`self.GetOwner`)))
          ; Get nearest smoke emitter
          (if (< _returnvalue (`local.ClosestDistance`))
            (set `local.NearestEmitter` _array_element)
            (set `local.ClosestDistance` _returnvalue)))))
    ; Add emitter to connected emitter if valid // remove connecting emitter from search array // reset local variables for further checks
    (if (`KismetSystemLibrary.IsValid` (`local.NearestEmitter`))
      (`self.ConnectEmitter` (`local.NearestEmitter`))
      (`KismetArrayLibrary.Array_RemoveItem` (`local.Emitters`) (`local.NearestEmitter`)))
    (set `local.ClosestDistance` (`self.MaxEmitterConnectDistance`))
    (set `local.NearestEmitter` null)))

(fn `DisconnectEmitter`
  (params (EmitterToDisconnect :type "/Game/PlaneContent/Blueprints/Physics/Smoke/Actor_SmokeEmitter Object Reference"))
  (locals (SuccessDisconnecting :type Boolean))
  (if (`KismetSystemLibrary.IsValid` EmitterToDisconnect)
    (if (`KismetArrayLibrary.Array_Contains` (`self.ConnectedSmokeEmitter`) (`local.EmitterToDisconnect`))
      (set `local.SuccessDisconnecting` false)
      (for _array_element (`self.LastSmokeAmoutsStengthAddedToSmokeEmitter`)
        (bind (_smokeemitter _lastsmokestrength) (break `/Game/PlaneContent/Blueprints/Physics/Smoke/St_SmokeSource` _array_element))
        (if (== (`local.EmitterToDisconnect`) _smokeemitter)
          (`/Game/PlaneContent/Blueprints/Physics/Smoke/Actor_SmokeEmitter.DecreaseSmokeValue` (`local.EmitterToDisconnect`) _lastsmokestrength)
          (`KismetArrayLibrary.Array_RemoveItem` (`self.LastSmokeAmoutsStengthAddedToSmokeEmitter`) _array_element)
          (`KismetArrayLibrary.Array_RemoveItem` (`self.ConnectedSmokeEmitter`) (`local.EmitterToDisconnect`))
          (`self.UpdateSmokeValueInEmitter`)
          (set `local.SuccessDisconnecting` true)
          (break)))
      (if (not (`local.SuccessDisconnecting`))
        (`KismetSystemLibrary.PrintString` (`KismetStringLibrary.Concat_StrStr` (`KismetSystemLibrary.GetDisplayName` (`self.GetOwner`)) ": " "Disconnectint Smoke Source from emitter went wrong") true true (struct :`G` 0.66 :`B` 1.0 :`A` 1.0) 8.0))
      (else
        (`KismetSystemLibrary.PrintString` (`KismetStringLibrary.Concat_StrStr` (`KismetSystemLibrary.GetDisplayName` (`self.GetOwner`)) ": " "Tried to disconnect NOT-CONNECTED Emitter from Smoke Source Component") true true (struct :`G` 0.66 :`B` 1.0 :`A` 1.0) 8.0)))
    (else
      (`KismetSystemLibrary.PrintString` (`KismetStringLibrary.Concat_StrStr` (`KismetSystemLibrary.GetDisplayName` (`self.GetOwner`)) ": " "Tried to disconnect non-valid Emitter from Smoke Source Component") true true (struct :`G` 0.66 :`B` 1.0 :`A` 1.0) 8.0))))

(fn `DrawDebugLines`
  (`|ExecutionSequence`
    (:`then_0`
      (if (`self.DebugLineToConnectedSmokeEmitter`)
        (`self.DrawDebugLineToConnectedSmokeEmitter` (`GameplayStatics.GetWorldDeltaSeconds`))))))

(fn `DrawDebugLineToConnectedSmokeEmitter`
  (params (DeltaTime :type "Float (double-precision)"))
  (if (not (`KismetArrayLibrary.Array_IsEmpty` (`self.ConnectedSmokeEmitter`)))
    (for _array_element (`self.ConnectedSmokeEmitter`)
      (`KismetSystemLibrary.DrawDebugLine` (`Actor.K2_GetActorLocation` (`self.GetOwner`)) (`Actor.K2_GetActorLocation` _array_element) (struct :`R` 1.0 :`A` 1.0) (* (`local.DeltaTime`) 2.0) 0.5)
      (bind _realsmokestrength (`self.GetRealSmokeStrength` _array_element))
      (bind _returnvalue (`Actor.K2_GetActorLocation` _array_element))
      (`KismetSystemLibrary.DrawDebugString` (+ (+ (/ (- (`Actor.K2_GetActorLocation` (`self.GetOwner`)) _returnvalue) 2.0) _returnvalue) (0.0 0.0 10.0)) (`KismetStringLibrary.Conv_DoubleToString` (`KismetMathLibrary.SelectFloat` (`self.SmokeStrength`) _realsmokestrength (== (`KismetArrayLibrary.Array_Length` (`self.ConnectedSmokeEmitter`)) 1))) null (struct :`R` 1.0 :`A` 1.0) (* (`local.DeltaTime`) 2.0)))))

(fn `GetRealSmokeStrength`
  (params (EmitterToConsider :type "/Game/PlaneContent/Blueprints/Physics/Smoke/Actor_SmokeEmitter Object Reference"))
  (returns (RealSmokeStrength :type "Float (double-precision)"))
  (locals (DistanceOfAllEmittersSquared :type "Float (double-precision)"))
  (if (not (`KismetArrayLibrary.Array_IsEmpty` (`self.ConnectedSmokeEmitter`)))
    (set `local.DistanceOfAllEmittersSquared` 0.0)
    (for _array_element (`self.ConnectedSmokeEmitter`)
      (set `local.DistanceOfAllEmittersSquared` (+ (`local.DistanceOfAllEmittersSquared`) (/ 1.0 (`KismetMathLibrary.Vector_DistanceSquared` (`Actor.K2_GetActorLocation` _array_element) (`Actor.K2_GetActorLocation` (`self.GetOwner`)))))))
    (return (* (/ (/ 1.0 (`KismetMathLibrary.Vector_DistanceSquared` (`Actor.K2_GetActorLocation` (`local.EmitterToConsider`)) (`Actor.K2_GetActorLocation` (`self.GetOwner`)))) (`local.DistanceOfAllEmittersSquared`)) (`self.SmokeStrength`)))))

(fn `UpdateConnectedEmitter`
  (locals (NotConnectedEmitters :type "Array of /Game/PlaneContent/Blueprints/Physics/Smoke/Actor_SmokeEmitter Object Reference") (EmittersQueuedForDisconnecting :type "Array of /Game/PlaneContent/Blueprints/Physics/Smoke/Actor_SmokeEmitter Object Reference") (NearestNonConnectedEmitter :type "/Game/PlaneContent/Blueprints/Physics/Smoke/Actor_SmokeEmitter Object Reference") (ClosestDistance :type "Float (single-precision)") (FurthestDistance :type "Float (double-precision)") (FurthestConnectedEmitter :type "/Game/PlaneContent/Blueprints/Physics/Smoke/Actor_SmokeEmitter Object Reference") (SearchIndex :type Integer) (EmitterQueuedForConnecting :type "Array of /Game/PlaneContent/Blueprints/Physics/Smoke/Actor_SmokeEmitter Object Reference") (NotConnectedBuffer :type "Array of /Game/PlaneContent/Blueprints/Physics/Smoke/Actor_SmokeEmitter Object Reference") (CompareIndex :type Integer))
  (set `self.LastPositionEmitterDetectionTick` (`Actor.K2_GetActorLocation` (`self.GetOwner`)))
  ;[0.15 0 0 0.5] Would also check for emitter through walls / Raycast would fix this / Better would be just to consider emitters which are in the same room as the smoke source so no raycast or extra checks are necessary
  (bind _outactors (`GameplayStatics.GetAllActorsOfClass` "/Game/PlaneContent/Blueprints/Physics/Smoke/Actor_SmokeEmitter.Actor_SmokeEmitter_C")) ; Change to actors from room
  (set `local.NotConnectedEmitters` _outactors)
  ; Filter out already connected emitters
  (for _array_element (`self.ConnectedSmokeEmitter`)
    (if (`KismetArrayLibrary.Array_Contains` (`local.NotConnectedEmitters`) _array_element)
      (`KismetArrayLibrary.Array_RemoveItem` (`local.NotConnectedEmitters`) _array_element)))
  (`|ExecutionSequence`
    (:`then_0`
      ; Disconnect Emitter which got out of range
      (for _array_element_2 (`self.ConnectedSmokeEmitter`)
        (if (not (`self.CheckIfEmitterIsInRange` _array_element_2))
          (`KismetArrayLibrary.Array_Add` (`local.EmittersQueuedForDisconnecting`) _array_element_2)))
      (if (`KismetArrayLibrary.Array_IsNotEmpty` (`local.EmittersQueuedForDisconnecting`))
        (for _array_element_3 (`local.EmittersQueuedForDisconnecting`)
          (`self.DisconnectEmitter` _array_element_3))
        (`KismetArrayLibrary.Array_Clear` (`local.EmittersQueuedForDisconnecting`))))
    (:`then_1`
      (set `local.CompareIndex` (`KismetArrayLibrary.Array_Length` (`self.ConnectedSmokeEmitter`)))
      (for _ (range 1 (+ (`self.MaxEmitterConnectionCount`) 1))
        (set `local.NotConnectedBuffer` (`local.NotConnectedEmitters`))
        (`|ExecutionSequence`
          (:`then_0`
            (set `local.ClosestDistance` (`self.MaxEmitterConnectDistance`))
            (for _array_element_4 (`local.NotConnectedBuffer`)
              ; Check if emitter is in range
              (if (`self.CheckIfEmitterIsInRange` _array_element_4)
                (bind _returnvalue (`Actor.GetDistanceTo` _array_element_4 (`self.GetOwner`)))
                ; Get nearest NOT-Connected smoke emitter
                (if (< _returnvalue (`local.ClosestDistance`))
                  (set `local.NearestNonConnectedEmitter` _array_element_4)
                  (set `local.ClosestDistance` _returnvalue)))))
          (:`then_1`
            (set `local.FurthestDistance` 0.0)
            (for _array_element_5 (`self.ConnectedSmokeEmitter`)
              (bind _returnvalue_2 (`Actor.GetDistanceTo` _array_element_5 (`self.GetOwner`)))
              ; Get furthest Connected smoke emitter
              (if (> _returnvalue_2 (`local.FurthestDistance`))
                (set `local.FurthestConnectedEmitter` _array_element_5)
                (set `local.FurthestDistance` _returnvalue_2))))
          (:`then_2`
            (if (not (< (`local.CompareIndex`) (`self.MaxEmitterConnectionCount`)))
              ; Switch connected emitter with non-connected emitter because it's closer to an emitter then the connected one
              (if (< (`local.ClosestDistance`) (`local.FurthestDistance`))
                (`KismetArrayLibrary.Array_Add` (`local.EmittersQueuedForDisconnecting`) (`local.FurthestConnectedEmitter`))
                (`KismetArrayLibrary.Array_Add` (`local.EmitterQueuedForConnecting`) (`local.NearestNonConnectedEmitter`))
                (`KismetArrayLibrary.Array_RemoveItem` (`local.NotConnectedEmitters`) (`local.NearestNonConnectedEmitter`))
                (`/Engine/EditorBlueprintResources/StandardMacros.IncrementInt` (`local.CompareIndex`)))
              (else
                ; Fill Connected Emitter array
                (if (`KismetSystemLibrary.IsValid` (`local.NearestNonConnectedEmitter`))
                  (`KismetArrayLibrary.Array_Add` (`local.EmitterQueuedForConnecting`) (`local.NearestNonConnectedEmitter`))
                  (if (`KismetSystemLibrary.IsValid` (`local.NearestNonConnectedEmitter`))
                    (`KismetArrayLibrary.Array_RemoveItem` (`local.NotConnectedEmitters`) (`local.NearestNonConnectedEmitter`))
                    (`/Engine/EditorBlueprintResources/StandardMacros.IncrementInt` (`local.CompareIndex`)))))))))
      ; Apply detection
      (`|ExecutionSequence`
        (:`then_0`
          (for _array_element_6 (`local.EmittersQueuedForDisconnecting`)
            (`self.DisconnectEmitter` _array_element_6)))
        (:`then_1`
          (for _array_element_7 (`local.EmitterQueuedForConnecting`)
            (`self.ConnectEmitter` _array_element_7)))))))

(fn `UpdateSmokeValueInEmitter`
  (locals (CurrentEmitter :type "/Game/PlaneContent/Blueprints/Physics/Smoke/Actor_SmokeEmitter Object Reference") (CurrentSmokeSource :type "/Game/PlaneContent/Blueprints/Physics/Smoke/St_SmokeSource Structure") (NewSmokeStrength :type "Float (double-precision)" :default 0.0) (Buffer :type "Array of /Game/PlaneContent/Blueprints/Physics/Smoke/St_SmokeSource Structure"))
  (bind _currentemitter (`local.CurrentEmitter`))
  (bind _newsmokestrength (`local.NewSmokeStrength`))
  (set `local.Buffer` (`self.LastSmokeAmoutsStengthAddedToSmokeEmitter`))
  (for _array_element (`local.Buffer`)
    (bind _output_get (set `local.CurrentSmokeSource` _array_element))
    (bind (_smokeemitter _lastsmokestrength) (break `/Game/PlaneContent/Blueprints/Physics/Smoke/St_SmokeSource` _output_get))
    (set `local.CurrentEmitter` _smokeemitter)
    (set `local.NewSmokeStrength` 0.0)
    (`|ExecutionSequence`
      (:`then_0`
        ; Remove old value from emitter
        (`/Game/PlaneContent/Blueprints/Physics/Smoke/Actor_SmokeEmitter.DecreaseSmokeValue` (`local.CurrentEmitter`) _lastsmokestrength))
      (:`then_1`
        ; Calculate new smoke value and replace in array
        (bind _realsmokestrength (`self.GetRealSmokeStrength` (`local.CurrentEmitter`)))
        (set `local.NewSmokeStrength` _realsmokestrength)
        (`KismetArrayLibrary.Array_RemoveItem` (`self.LastSmokeAmoutsStengthAddedToSmokeEmitter`) (`local.CurrentSmokeSource`))
        (`KismetArrayLibrary.Array_Add` (`self.LastSmokeAmoutsStengthAddedToSmokeEmitter`) (make `/Game/PlaneContent/Blueprints/Physics/Smoke/St_SmokeSource` (`local.CurrentEmitter`) (`local.NewSmokeStrength`))))
      (:`then_2`
        ; Apply new smoke strength to emitter
        (`/Game/PlaneContent/Blueprints/Physics/Smoke/Actor_SmokeEmitter.IncreaseSmokeValue` _currentemitter _newsmokestrength)
        (`KismetSystemLibrary.PrintString` (`KismetStringLibrary.Concat_StrStr` "Add Smoke Value: " (`KismetStringLibrary.Conv_DoubleToString` _newsmokestrength) " (" (`KismetSystemLibrary.GetDisplayName` _currentemitter) ")") true true (struct :`G` 0.66 :`B` 1.0 :`A` 1.0) (`self.UpdateSmokeStrengthTick`))))))