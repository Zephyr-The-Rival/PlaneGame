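; Liquid spawner actor that creates BP_Liquid actors at its own transform and keeps track of them.
; BeginPlay starts a fast looping timer, and SpawnLiquidActor spawns one liquid actor per call, adding it to an array.
; Reset destroys every tracked liquid actor and clears the array, leaving the timer untouched.
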(event `self.ReceiveBeginPlay`
  (`KismetSystemLibrary.K2_SetTimerDelegate` (`|CreateDelegate` :!event `SpawnLiquidActor`) 0.1 true))

(event `Reset`
  (for _array_element (`self.Array`)
    (`self.K2_DestroyActor` _array_element))
  (`KismetArrayLibrary.Array_Clear` (`self.Array`)))

(event `SpawnLiquidActor`
  (bind _returnvalue (`|SpawnActorFromClass` "/Game/PlaneContent/Blueprints/Systems/Liquid/BP_Liquid.BP_Liquid_C" (`self.GetTransform`) "Undefined" "MultiplyWithRoot" null null))
  (`KismetArrayLibrary.Array_Add` (`self.Array`) _returnvalue))

(fn `UserConstructionScript`)