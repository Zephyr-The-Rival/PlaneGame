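; BP_Lever is a networked hold-to-interact lever that a player drags by hand, outputting a 0–1 value through OnLeverMoved.
; While held, the server maps the hand's position relative to the base to that value, releasing it beyond a distance limit.
; Optional thresholds snap it to either end and force release, while an optional timeline eases unsnapped levers back to the start value.
; Handle rotation is multicast to clients.
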(event `self.HoldInteract_Start`
  (params (InteractingPlayer :type "PlanePlayerCharacter Object Reference"))
  ; InteractStart
  (`parent.HoldInteract_Start` InteractingPlayer)
  (`|ExecutionSequence`
    (:`then_0`
      (set `self.InteractingPlayer` InteractingPlayer)
      (set `self.BeeingUsed` true)
      (set `self.CurrentValue` (`self.StartValue`)))
    (:`then_1`
      (`PrimitiveComponent.SetCollisionEnabled` (`self.Sphere`) "NoCollision"))
    (:`then_2`
      (if (`self.MoveBackToStartValueOnLetGo`)
        (`self.StopMoveBack`)))))

(event `self.HoldInteract_End`
  (params (InteractingPlayer :type "PlanePlayerCharacter Object Reference"))
  ; InteractEnd
  (`parent.HoldInteract_End` InteractingPlayer)
  (`|ExecutionSequence`
    (:`then_0`
      (set `self.BeeingUsed` false))
    (:`then_1`
      (`PrimitiveComponent.SetCollisionEnabled` (`self.Sphere`) "QueryOnly"))
    (:`then_2`
      (if (and (`self.MoveBackToStartValueOnLetGo`) (not (or (and (`self.SnapTop`) (== (`self.CurrentValue`) 1.0)) (and (`self.SnapBottom`) (== (`self.CurrentValue`) 0.0)))))
        (`self.StartMoveBack`)))))

(event `StartMoveBack`
  ; Move Back
  (bind (_direction _0_1) (`Timeline|MoveBackTimeline` :!via `PlayFromStart` :!label _label)
    (:`Update`
      (set `self.CurrentValue` (`KismetMathLibrary.Lerp` (`self.LastValue`) (`self.StartValue`) _0_1))
      (`self.ApplyValue`))))

(event `StopMoveBack`
  ; Move Back
  (goto _label :!via `Stop`))

(event `Multicast_SetHandleRotation`
  (params (Value :type "Float (double-precision)"))
  (`self.SetHandleByValue` Value))

(event `self.ReceiveTick`
  (params (DeltaSeconds :type "Float (single-precision)"))
  (bind _snapbottomthreshold (`self.SnapBottomThreshold`))
  (bind _snaptopthreshold (`self.SnapTopThreshold`))
  (bind _returnvalue_location (`KismetMathLibrary.BreakTransform` (`KismetMathLibrary.MakeRelativeTransform` (`SceneComponent.K2_GetComponentToWorld` (`Actor.RootComponent` (`PlanePlayerCharacter.MyPlayerHand` (`self.InteractingPlayer`)))) (`SceneComponent.K2_GetComponentToWorld` (`self.Base`)))))
  (`/Engine/EditorBlueprintResources/ActorMacros.Switch Has Authority`
    (:`Authority`
      ; While Beeing Used
      (if (`self.BeeingUsed`)
        (if (not (> (`KismetMathLibrary.Vector_Distance` (`SceneComponent.K2_GetComponentLocation` (`self.Sphere`)) (`SceneComponent.K2_GetComponentLocation` (`Actor.RootComponent` (`PlanePlayerCharacter.MyPlayerHand` (`self.InteractingPlayer`))))) (`self.LetGoDistance`)))
          (`|ExecutionSequence`
            (:`then_0`
              (set `self.CurrentValue` (`KismetMathLibrary.FClamp` (/ (+ (* (.x _returnvalue_location) 1.5) 60.0) 120.0))))
            (:`then_1`
              (if (`self.SnapTop`)
                (if (and (> (`self.CurrentValue`) _snaptopthreshold) (< (`self.LastValue`) _snaptopthreshold))
                  (set `self.CurrentValue` 1.0)
                  (`self.ApplyValue`)
                  (`PlanePlayerCharacter.LetGoHoldInteract` (`self.InteractingPlayer`)))))
            (:`then_2`
              (if (`self.SnapBottom`)
                (if (and (< (`self.CurrentValue`) _snapbottomthreshold) (> (`self.LastValue`) _snapbottomthreshold))
                  (set `self.CurrentValue` 0.0)
                  (`self.ApplyValue`)
                  (`PlanePlayerCharacter.LetGoHoldInteract` (`self.InteractingPlayer`)))))
            (:`then_3`
              (`self.ApplyValue`))
            (:`then_4`
              (set `self.LastValue` (`self.CurrentValue`))))
          (else
            (`PlanePlayerCharacter.LetGoHoldInteract` (`self.InteractingPlayer`))))))))

(fn `ApplyValue`
  (`self.Multicast_SetHandleRotation` (`self.CurrentValue`))
  (`self.OnLeverMoved` (`self.CurrentValue`)))

(fn `SetHandleByValue`
  (params (Value :type "Float (double-precision)"))
  (`SceneComponent.K2_SetRelativeRotation` (`self.Handle`) (`KismetMathLibrary.MakeRotator` 0.0 (`KismetMathLibrary.Lerp` 60.0 -60.0 Value)) false false))

(fn `UserConstructionScript`
  (`self.SetHandleByValue` (`self.StartValue`)))