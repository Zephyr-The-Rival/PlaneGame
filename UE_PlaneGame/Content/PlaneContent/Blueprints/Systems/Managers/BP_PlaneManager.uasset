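; Plane manager that fills the plane's seat rows with passenger NPCs over time, run with authority.
; After a short delay it reads floors from BP_RoomManager and records each seat row's capacity by row class, grouped by room.
; A looping timer has random rows create NPCs, dropping full rows and empty rooms until the passenger target or capacity is reached.
; A separate helper finds random reachable points around spawn points.
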(event `self.ReceiveBeginPlay`
  (if (`self.HasAuthority` (`GameplayStatics.GetPlayerController` 0))
    (`KismetSystemLibrary.Delay` 1.0)
    (bind _returnvalue (`GameplayStatics.GetActorOfClass` "/Game/PlaneContent/Blueprints/Systems/Managers/RoomManager/BP_RoomManager.BP_RoomManager_C"))
    (set `self.Floors` (`/Game/PlaneContent/Blueprints/Systems/Managers/RoomManager/BP_RoomManager.Floors` _returnvalue))
    (`|ExecutionSequence`
      (:`then_0`
        ; Spawn Passenger
        (`self.PrepairPassengerSpawning`)
        (if (> (`KismetArrayLibrary.Array_Length` (`self.Rooms with Stats`)) 0)
          (bind _returnvalue_2 (`KismetSystemLibrary.K2_SetTimerDelegate` (`|CreateDelegate` :!event `StartSpawningPassengers`) (`self.SpawnInterval`) true))
          (set `self.SpawnPassengerTimer` _returnvalue_2))))))

(event `StartSpawningPassengers`
  ; Spawn Passenger
  (`self.SpawnPassenger`))

(fn `GetRandomSpawnPoint`
  (returns (SpawnLocation :type "Vector Structure"))
  (bind _outitem (`KismetArrayLibrary.Array_Random` (`self.SpawnPoints`)))
  (bind (_randomlocation _returnvalue) (`NavigationSystemV1.K2_GetRandomReachablePointInRadius` (`self.K2_GetActorLocation` _outitem) (`SphereComponent.GetScaledSphereRadius` (`/Game/PlaneContent/Blueprints/GameInstance/BP_SpawnPoint.Sphere` _outitem)) null null))
  (if (`KismetArrayLibrary.Array_IsNotEmpty` (`self.SpawnPoints`))
    (if _returnvalue
      (return _randomlocation)
      (else
        (`KismetSystemLibrary.PrintString` "NO SPAWN LOCATION FOUNT (PLANE MANAGER)" true true (struct :`R` 1.0 :`G` 0.005 :`B` 0.001 :`A` 1.0) 10.0)))
    (else
      (`KismetSystemLibrary.PrintString` "NO SPAWN POINTS IN PLANE MANAGER!!!" true true (struct :`R` 1.0 :`G` 0.005 :`B` 0.001 :`A` 1.0) 10.0))))

(fn `PrepairPassengerSpawning`
  (returns (RoomsWithStats :type "Array of /Game/PlaneContent/Blueprints/Systems/Managers/RoomManager/ST_RoomWithRowSpawnStats Structure"))
  (locals (RoomIndex :type Integer :default 0) (MaxPassenger :type Integer :default 0) (`Rooms with Seat Rows` :type "Array of /Game/PlaneContent/Blueprints/Systems/Managers/RoomManager/BP_Room Object Reference"))
  (set `self.SpawnedPassenger` 0)
  (`KismetArrayLibrary.Array_Clear` (`self.Rooms with Stats`))
  (`KismetArrayLibrary.Array_Clear` (`local.Rooms with Seat Rows`))
  (for _array_element (`self.Floors`)
    (for _array_element_2 (`.Rooms_3_A1BFCC0643B75667517BE88B738977A7` (break `/Game/PlaneContent/Blueprints/Systems/Managers/RoomManager/ST_Floor` _array_element))
      (if (> (`KismetArrayLibrary.Array_Length` (`/Game/PlaneContent/Blueprints/Systems/Managers/RoomManager/BP_Room.SeatRowsInRoom` _array_element_2)) 0)
        (`KismetArrayLibrary.Array_AddUnique` (`local.Rooms with Seat Rows`) _array_element_2))))
  (if (> (`KismetArrayLibrary.Array_Length` (`local.Rooms with Seat Rows`)) 0)
    (for _array_element_3 (`local.Rooms with Seat Rows`)
      (bind _returnvalue (`KismetArrayLibrary.Array_Add` (`self.Rooms with Stats`) (make `/Game/PlaneContent/Blueprints/Systems/Managers/RoomManager/ST_RoomWithRowSpawnStats` _array_element_3)))
      (set `local.RoomIndex` _returnvalue)
      (for _array_element_4 (`/Game/PlaneContent/Blueprints/Systems/Managers/RoomManager/BP_Room.SeatRowsInRoom` _array_element_3)
        (cast `/Game/PlaneContent/Blueprints/Systems/PlaneActors/SeatRows/SeatRow_1S` _array_element_4
          (:`then`
            (set `local.MaxPassenger` 1)
            (`KismetArrayLibrary.Array_Add` (`.SpawnStats_8_E5666E72483A9DB917F64E91426EB425` (break `/Game/PlaneContent/Blueprints/Systems/Managers/RoomManager/ST_RoomWithRowSpawnStats` (`|GetArrayItem` (`self.Rooms with Stats`) (`local.RoomIndex`)))) (make `/Game/PlaneContent/Blueprints/Systems/Managers/RoomManager/ST_SpawmRowStats` _array_element_4 (`local.MaxPassenger`)) :!label _label))
          (:`CastFailed`
            (cast `/Game/PlaneContent/Blueprints/Systems/PlaneActors/SeatRows/SeatRow_2S` _array_element_4
              (:`then`
                (set `local.MaxPassenger` 2)
                (goto _label))
              (:`CastFailed`
                (cast `/Game/PlaneContent/Blueprints/Systems/PlaneActors/SeatRows/SeatRow_3S` _array_element_4
                  (:`then`
                    (set `local.MaxPassenger` 3)
                    (goto _label))
                  (:`CastFailed`
                    (`KismetSystemLibrary.PrintString` "ERROR PREPAIRING PASSENGER SPAWN (BP SHIP MANAGER)" true true (struct :`R` 1.0 :`A` 1.0) 10.0)))))))))
    (return (`self.Rooms with Stats`))))

(fn `SpawnPassenger`
  (bind _index_stats (`self.Index Stats`))
  (bind ((`SpawnStats_8_E5666E72483A9DB917F64E91426EB425` _spawnstats)) (break `/Game/PlaneContent/Blueprints/Systems/Managers/RoomManager/ST_RoomWithRowSpawnStats` (`|GetArrayItem` (`self.Rooms with Stats`) (`self.IndexRoomWithStats`))))
  (bind _output (`|GetArrayItem` _spawnstats _index_stats))
  (bind (_seatrow _maxpassengers _spawnedcounter) (break `/Game/PlaneContent/Blueprints/Systems/Managers/RoomManager/ST_SpawmRowStats` _output))
  (if (or (== (`self.PassengerAmount`) (`self.SpawnedPassenger`)) (`KismetArrayLibrary.Array_IsEmpty` (`self.Rooms with Stats`)))
    (`KismetSystemLibrary.K2_ClearAndInvalidateTimerHandle` (`self.SpawnPassengerTimer`))
    (else
      (set `self.IndexRoomWithStats` (`KismetMathLibrary.RandomIntegerInRange` 0 (- (`KismetArrayLibrary.Array_Length` (`self.Rooms with Stats`)) 1)))
      (set `self.Index Stats` (`.OutIndex` (`KismetArrayLibrary.Array_Random` _spawnstats)))
      (`/Game/PlaneContent/Blueprints/Systems/PlaneActors/SeatRows/Base/ActorPassengerSeatRow.CreateNpc` _seatrow)
      (`/Engine/EditorBlueprintResources/StandardMacros.IncrementInt` (`self.SpawnedPassenger`)
        (:`  `
          (bind _result (`/Engine/EditorBlueprintResources/StandardMacros.IncrementInt` _spawnedcounter)
            (:`  `
              (if (>= _result _maxpassengers)
                ; Remove full row
                (`KismetArrayLibrary.Array_Remove` (`.SpawnStats_8_E5666E72483A9DB917F64E91426EB425` (break `/Game/PlaneContent/Blueprints/Systems/Managers/RoomManager/ST_RoomWithRowSpawnStats` (`|GetArrayItem` (`self.Rooms with Stats`) (`self.IndexRoomWithStats`)))) _index_stats)
                ; Remove room with no spawns left
                (if (`KismetArrayLibrary.Array_IsEmpty` (`.SpawnStats_8_E5666E72483A9DB917F64E91426EB425` (break `/Game/PlaneContent/Blueprints/Systems/Managers/RoomManager/ST_RoomWithRowSpawnStats` (`|GetArrayItem` (`self.Rooms with Stats`) (`self.IndexRoomWithStats`)))))
                  (`KismetArrayLibrary.Array_RemoveItem` (`self.Rooms with Stats`) (`|GetArrayItem` (`self.Rooms with Stats`) (`self.IndexRoomWithStats`))))
                (else
                  (setmembers `/Game/PlaneContent/Blueprints/Systems/Managers/RoomManager/ST_SpawmRowStats` :`StructRef` _output :`SpawnedCounter` _result))))))))))

(fn `UserConstructionScript`)