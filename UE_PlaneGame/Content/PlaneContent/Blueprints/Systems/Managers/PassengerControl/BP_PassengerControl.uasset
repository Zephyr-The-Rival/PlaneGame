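; Passenger control manager that caps how many passenger need requests of each type can be active at once.
; On BeginPlay it builds a per-need collection from the enum, taking limits from the NeedSettings DataTable by row index, so row order must match enum order.
; RequestNeedDemand increments the count and grants requests below the limit.
; A looping minute timer accompanies ResetCollection, which zeroes all active counts.
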(event `self.ReceiveBeginPlay`
  (`self.SetUpCollection`)
  (`KismetSystemLibrary.K2_SetTimerDelegate` (`|CreateDelegate` :!event `ResetCollection`) 60.0 true))

(event `ResetCollection`
  (for (_ _array_index) (`self.Collection`)
    (setmembers `/Game/PlaneContent/Blueprints/Systems/Managers/PassengerControl/ST_MaxActiveNeed` :`StructRef` (`|GetArrayItem` (`self.Collection`) _array_index) :`CurrentlyActive` 0)))

(fn `RequestNeedDemand`
  (params (RequestedNeed :type "/Game/PlaneContent/Blueprints/Systems/Passenger/Components/Needs/Enum_PassengerNeeds Enum" :default "NewEnumerator6"))
  (returns (RequestAccepted :type Boolean))
  (if (`KismetArrayLibrary.Array_IsNotEmpty` (`self.Collection`))
    (for (_array_element _array_index) (`self.Collection`)
      (if (`|EnumEquality` (`.Need_2_0ECFC9BF4A78F339DE8888A840934A6F` (break `/Game/PlaneContent/Blueprints/Systems/Managers/PassengerControl/ST_MaxActiveNeed` _array_element)) (`local.RequestedNeed`))
        (bind _output (`|GetArrayItem` (`self.Collection`) _array_index))
        (bind (_need _maxactiveneed _currentlyactive) (break `/Game/PlaneContent/Blueprints/Systems/Managers/PassengerControl/ST_MaxActiveNeed` _output))
        (if (> _currentlyactive _maxactiveneed)
          (`KismetSystemLibrary.PrintString` (`KismetStringLibrary.Concat_StrStr` "MORE NEED REQUEST ACTIVE THAN ALLOWED (" (`|GetEnumeratorNameAsString` _need) ")") true true (struct :`R` 1.0 :`G` 0.021865 :`A` 1.0) 10.0)
          (elif (< _currentlyactive _maxactiveneed)
            (bind _result (`/Engine/EditorBlueprintResources/StandardMacros.IncrementInt` _currentlyactive)
              (:`  `
                (setmembers `/Game/PlaneContent/Blueprints/Systems/Managers/PassengerControl/ST_MaxActiveNeed` :`StructRef` _output :`CurrentlyActive` _result)
                (return true)))
            (else
              (return false))))))
    (return false)
    (else
      (return false))))

(fn `SetUpCollection`
  (`/Engine/EditorBlueprintResources/StandardMacros.IsValid` (`self.NeedSettings`)
    (:`Is Valid`
      (bind _enumvalue (foreach `/Game/PlaneContent/Blueprints/Systems/Passenger/Components/Needs/Enum_PassengerNeeds` true)
        (:`LoopBody`
          (if (`|EnumInequality` _enumvalue "NewEnumerator6")
            (`KismetArrayLibrary.Array_AddUnique` (`self.Collection`) (make `/Game/PlaneContent/Blueprints/Systems/Managers/PassengerControl/ST_MaxActiveNeed` _enumvalue))))
        (:`then`
          (bind _outrownames (`DataTableFunctionLibrary.GetDataTableRowNames` (`self.NeedSettings`)))
          (for (_array_element _array_index) _outrownames
            (bind _returnvalue (`|GetDataTableRow` (`self.NeedSettings`) _array_element)
              (:`then`
                (bind (_need _maxactiveneed) (break `/Game/PlaneContent/Blueprints/Systems/Managers/PassengerControl/ST_MaxActiveNeed` _returnvalue))
                (if (`|EnumInequality` _need "NewEnumerator6")
                  (setmembers `/Game/PlaneContent/Blueprints/Systems/Managers/PassengerControl/ST_MaxActiveNeed` :`StructRef` (`|GetArrayItem` (`self.Collection`) _array_index) :`MaxActiveNeed` _maxactiveneed))))))))
    (:`Is Not Valid`
      (`KismetSystemLibrary.PrintString` (`KismetStringLibrary.Concat_StrStr` "PASSENGER CONTROL HAS NO NEED SETTINGS SET (DATA TABLE)") true true (struct :`R` 1.0 :`A` 1.0) 10.0))))

(fn `UserConstructionScript`)