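; BP_Room is a room in the plane that tracks its passenger seat rows and the components that can satisfy each passenger need.
; On BeginPlay it finds BP_RoomManager, prints a red warning if the room is missing from the manager's floor arrays, and creates one target entry per need enum value except one.
; Registering room components receive a reference to the room, and need target components are filed under their matching need.
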(event `self.ReceiveBeginPlay`
  (`self.Init`)
  (`self.CheckIfRoomIsInRoomManager`)
  (bind _enumvalue (foreach `/Game/PlaneContent/Blueprints/Systems/Passenger/Components/Needs/Enum_PassengerNeeds` false)
    (:`LoopBody`
      (if (`|EnumInequality` _enumvalue "NewEnumerator6")
        (`KismetArrayLibrary.Array_AddUnique` (`self.NeedTargets`) (make `/Game/PlaneContent/Blueprints/Systems/Managers/RoomManager/ST_NeedTargets` _enumvalue))))))

(event `RegisterToRoom`
  (params (RoomComponent :type "/Game/PlaneContent/Blueprints/Systems/Managers/RoomManager/RoomComponent Object Reference"))
  (bind _asactor_passenger_seat_row (cast `/Game/PlaneContent/Blueprints/Systems/PlaneActors/SeatRows/Base/ActorPassengerSeatRow` (`ActorComponent.GetOwner` RoomComponent))
    (:`then`
      (`KismetArrayLibrary.Array_AddUnique` (`self.SeatRowsInRoom`) _asactor_passenger_seat_row))
    (:`CastFailed`
      _))
  (set `/Game/PlaneContent/Blueprints/Systems/Managers/RoomManager/RoomComponent.Room` self RoomComponent))

(fn `CheckIfRoomIsInRoomManager`
  (locals (RoomInManager :type Boolean))
  (for _array_element (`/Game/PlaneContent/Blueprints/Systems/Managers/RoomManager/BP_RoomManager.Floors` (`self.RoomManager`))
    (for _array_element_2 (`.Rooms_3_A1BFCC0643B75667517BE88B738977A7` (break `/Game/PlaneContent/Blueprints/Systems/Managers/RoomManager/ST_Floor` _array_element))
      (if (== _array_element_2 self)
        (set `local.RoomInManager` true)
        (break)))
    (if (`local.RoomInManager`)
      (break)))
  (if (not (`local.RoomInManager`))
    (`KismetSystemLibrary.PrintString` (`KismetStringLibrary.Concat_StrStr` "ROOM NOT IN FLOOR ARRAY OF ROOM MANAGER (" (`KismetSystemLibrary.GetDisplayName` self) ")") true true (struct :`R` 1.0 :`A` 1.0) 10.0)))

(fn `Init`
  (bind _returnvalue (`GameplayStatics.GetActorOfClass` "/Game/PlaneContent/Blueprints/Systems/Managers/RoomManager/BP_RoomManager.BP_RoomManager_C"))
  (`/Engine/EditorBlueprintResources/StandardMacros.IsValid` _returnvalue
    (:`Is Valid`
      (set `self.RoomManager` _returnvalue))))

(fn `RegisterAsNeedTarget`
  (params (Need :type "/Game/PlaneContent/Blueprints/Systems/Passenger/Components/Needs/Enum_PassengerNeeds Enum" :default "NewEnumerator6") (NeedTargetComponent :type "/Game/PlaneContent/Blueprints/Systems/PlaneActors/NeedActors/NeedTargetComponent Object Reference"))
  (for (_array_element _array_index) (`self.NeedTargets`)
    (if (`|EnumEquality` (`.Need_3_989B239D484EA0AC72D019981388CB9E` (break `/Game/PlaneContent/Blueprints/Systems/Managers/RoomManager/ST_NeedTargets` _array_element)) Need)
      (`KismetArrayLibrary.Array_Add` (`.Components_6_72865D4746AC18AFB6203BAA7E3A7A9B` (break `/Game/PlaneContent/Blueprints/Systems/Managers/RoomManager/ST_NeedTargets` (`|GetArrayItem` (`self.NeedTargets`) _array_index))) (`local.NeedTargetComponent`)))))

(fn `UserConstructionScript`)