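; Elevator controller actor, filed under NotWorking, that spawns a chain of BP_ElevatorCabin actors along a looping-movement path.
; Spawn builds a four-point linear spline, recomputes even cabin spacing from its length, then spawns cabins along it.
; Each cabin's InterpToMovement gets the loop duration and control points, though middle points are zero vectors.
; BeginPlay and the construction script are empty; older path-setup and restart logic sits disconnected.
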(event `self.ReceiveBeginPlay`)

(event `Spawn`
  (bind _returnvalue (`KismetMathLibrary.FFloor` (/ (`SplineComponent.GetSplineLength` (`self.Spline`)) (+ (`self.DistanceBetweenCabins`) (`self.CabinHeight`)))))
  (`SplineComponent.ClearSplinePoints` (`self.Spline`) true)
  (`SplineComponent.AddSplinePoint` (`self.Spline`) (`self.Pos1`) "Local" true)
  (`SplineComponent.AddSplinePoint` (`self.Spline`) (`self.Pos2`) "Local" true)
  (`SplineComponent.AddSplinePoint` (`self.Spline`) (`self.Pos3`) "Local" true)
  (`SplineComponent.AddSplinePoint` (`self.Spline`) (`self.Pos4`) "Local" true)
  (for _index (range 4)
    (`SplineComponent.SetSplinePointType` (`self.Spline`) _index "Linear" true))
  (set `self.CurrentSpawnDistance` 0.0)
  (set `self.DistanceBetweenCabins` (/ (- (`SplineComponent.GetSplineLength` (`self.Spline`)) (* (`self.CabinHeight`) _returnvalue)) _returnvalue))
  (for _ (range (+ _returnvalue 1))
    (bind _returnvalue_2 (`|SpawnActorFromClass` "/Game/PlaneContent/Blueprints/Systems/PlaneActors/Elevator/BP_ElevatorCabin.BP_ElevatorCabin_C" (`KismetMathLibrary.MakeTransform` (`SplineComponent.GetLocationAtDistanceAlongSpline` (`self.Spline`) (`self.CurrentSpawnDistance`) "World")) "Undefined" "MultiplyWithRoot" null null))
    (set `self.CurrentSpawnDistance` (+ (`self.CurrentSpawnDistance`) (+ (`self.DistanceBetweenCabins`) (`self.CabinHeight`))))
    (bind _returnvalue_3 (`self.GetComponentByClass` _returnvalue_2 "/Script/Engine.InterpToMovementComponent"))
    (set `InterpToMovementComponent.Duration` (`self.LoopDuration`) _returnvalue_3)
    (`InterpToMovementComponent.AddControlPointPosition` _returnvalue_3 (`SplineComponent.GetLocationAtDistanceAlongSpline` (`self.Spline`) (`self.CurrentSpawnDistance`) "World") false)
    (`InterpToMovementComponent.AddControlPointPosition` _returnvalue_3 (0.0 0.0 0.0) false)
    (`InterpToMovementComponent.AddControlPointPosition` _returnvalue_3 (0.0 0.0 0.0) false)
    (`InterpToMovementComponent.AddControlPointPosition` _returnvalue_3 (0.0 0.0 0.0) false)
    (`InterpToMovementComponent.AddControlPointPosition` _returnvalue_3 (0.0 0.0 0.0) false)
    (`InterpToMovementComponent.AddControlPointPosition` _returnvalue_3 (`SplineComponent.GetLocationAtDistanceAlongSpline` (`self.Spline`) (`self.CurrentSpawnDistance`) "World") false)))

(fn `UserConstructionScript`)