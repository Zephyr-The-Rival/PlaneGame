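; BP_ElevatorCabin is an elevator cabin actor with a Cube that opens or closes in response to overlaps with a Box trigger.
; When a BP_PlanePlayerCharacter enters the Box, the Cube is hidden and its collision is disabled.
; When an overlap ends and no actors of any class remain in the Box, the Cube becomes visible again with query and physics collision.
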(event `self.ReceiveBeginPlay`)

(event `self.Box.OnComponentBeginOverlap`
  (params (OverlappedComponent :type "PrimitiveComponent Object Reference") (OtherActor :type "Actor Object Reference") (OtherComp :type "PrimitiveComponent Object Reference") (OtherBodyIndex :type Integer) (bFromSweep :type Boolean) (SweepResult :type "HitResult Structure (by ref)"))
  (bind _cube (`self.Cube`))
  (cast `/Game/PlaneContent/Blueprints/PlayerCharacter/BP_PlanePlayerCharacter` OtherActor)
  (`SceneComponent.SetVisibility` _cube false false)
  (`PrimitiveComponent.SetCollisionEnabled` _cube "NoCollision"))

(event `self.Box.OnComponentEndOverlap`
  (params (OverlappedComponent :type "PrimitiveComponent Object Reference") (OtherActor :type "Actor Object Reference") (OtherComp :type "PrimitiveComponent Object Reference") (OtherBodyIndex :type Integer))
  (bind _cube (`self.Cube`))
  (if (== (`KismetArrayLibrary.Array_Length` (`PrimitiveComponent.GetOverlappingActors` (`self.Box`) null)) 0)
    (`SceneComponent.SetVisibility` _cube true false)
    (`PrimitiveComponent.SetCollisionEnabled` _cube "QueryAndPhysics")))

(fn `UserConstructionScript`)