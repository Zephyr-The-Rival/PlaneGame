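; Elevator spline actor that carries a chain of BP_ElevatorCabin actors along a spline, resembling a paternoster lift.
; On BeginPlay it spawns evenly spaced cabins, pre-rotating those in the end ranges, then starts moving after a short delay.
; Each Tick it advances every cabin by speed, recomputing spline distance from its current location.
; Distance windows around spline points 0–3, adjusted by offsets and cabin height, trigger cabin rotation and top contraction.
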(event `self.ReceiveBeginPlay`
  (`|ExecutionSequence`
    (:`then_0`
      (`self.SpawnCabinsAlongSpline`)
      (`KismetSystemLibrary.Delay` 0.2)
      (set `self.Active` true))))

(event `self.ReceiveTick`
  (params (DeltaSeconds :type "Float (single-precision)"))
  (if (`self.Active`)
    (for (_array_element _array_index) (`self.Cabins`)
      (`self.K2_SetActorLocation` _array_element (`SplineComponent.GetLocationAtDistanceAlongSpline` (`self.Spline`) (+ (`SplineComponent.GetDistanceAlongSplineAtLocation` (`self.Spline`) (`self.K2_GetActorLocation` _array_element) "World") (* (`self.Speed`) (`GameplayStatics.GetWorldDeltaSeconds`))) "World") false false)
      (bind _output (`|GetArrayItem` (`self.Cabins`) _array_index))
      (`self.CheckShouldCabinRotate` _output)
      (`self.CheckCabinTopShouldContract` _output))))

(event `CheckCabinTopShouldContract`
  (params (Cabin :type "/Game/PlaneContent/Blueprints/Systems/PlaneActors/Elevator/BP_ElevatorCabin Object Reference") (Shouldinstant :type Boolean))
  (`self.HandleCabinTopContraction` Cabin Shouldinstant))

(event `CheckShouldCabinRotate`
  (params (Cabin :type "/Game/PlaneContent/Blueprints/Systems/PlaneActors/Elevator/BP_ElevatorCabin Object Reference"))
  (bind _returnvalue (`SplineComponent.GetDistanceAlongSplineAtLocation` (`self.Spline`) (`self.K2_GetActorLocation` Cabin) "World"))
  (bind _returnvalue_2 (`SplineComponent.GetDistanceAlongSplineAtLocation` (`self.Spline`) (`self.K2_GetActorLocation` Cabin) "World"))
  (if (`/Game/PlaneContent/Blueprints/Systems/PlaneActors/Elevator/BP_ElevatorCabin.Rotated` Cabin)
    (if (and (< _returnvalue_2 (+ (`SplineComponent.GetDistanceAlongSplineAtSplinePoint` (`self.Spline`) 3) (`self.RotateOffsetDistnace`))) (> _returnvalue_2 (+ (`SplineComponent.GetDistanceAlongSplineAtSplinePoint` (`self.Spline`) 1) (`self.RotateOffsetDistnace`))))
      (`/Game/PlaneContent/Blueprints/Systems/PlaneActors/Elevator/BP_ElevatorCabin.Rotate` Cabin false false))
    (elif (or (< _returnvalue (`SplineComponent.GetDistanceAlongSplineAtSplinePoint` (`self.Spline`) 1)) (> _returnvalue (+ (`SplineComponent.GetDistanceAlongSplineAtSplinePoint` (`self.Spline`) 3) (`self.RotateOffsetDistnace`))))
      (`/Game/PlaneContent/Blueprints/Systems/PlaneActors/Elevator/BP_ElevatorCabin.Rotate` Cabin true false))))

(fn `HandleCabinTopContraction`
  (params (Cabin :type "/Game/PlaneContent/Blueprints/Systems/PlaneActors/Elevator/BP_ElevatorCabin Object Reference") (Instant :type Boolean))
  (bind _cabin (`local.Cabin`))
  (bind _cabin_2 (`local.Cabin`))
  (bind _returnvalue (`SplineComponent.GetDistanceAlongSplineAtSplinePoint` (`self.Spline`) 1))
  (bind _returnvalue_2 (`SplineComponent.GetDistanceAlongSplineAtSplinePoint` (`self.Spline`) 2))
  (bind _returnvalue_3 (`SplineComponent.GetDistanceAlongSplineAtSplinePoint` (`self.Spline`) 0))
  (bind _returnvalue_4 (`SplineComponent.GetDistanceAlongSplineAtSplinePoint` (`self.Spline`) 3))
  (bind _returnvalue_5 (`SplineComponent.GetDistanceAlongSplineAtLocation` (`self.Spline`) (`self.K2_GetActorLocation` _cabin_2) "World"))
  (bind _returnvalue_6 (`SplineComponent.GetDistanceAlongSplineAtLocation` (`self.Spline`) (`self.K2_GetActorLocation` _cabin_2) "World"))
  (bind _returnvalue_7 (`SplineComponent.GetDistanceAlongSplineAtLocation` (`self.Spline`) (`self.K2_GetActorLocation` _cabin) "World"))
  (bind _returnvalue_8 (`SplineComponent.GetDistanceAlongSplineAtLocation` (`self.Spline`) (`self.K2_GetActorLocation` _cabin) "World"))
  (if (`/Game/PlaneContent/Blueprints/Systems/PlaneActors/Elevator/BP_ElevatorCabin.Contracted` (`local.Cabin`))
    (if (and (< _returnvalue_8 (+ _returnvalue_3 (+ (`self.CabinHeight`) (`self.ContractOffsetDistance`)))) (> _returnvalue_8 (+ _returnvalue_3 (`self.CabinHeight`))))
      (`/Game/PlaneContent/Blueprints/Systems/PlaneActors/Elevator/BP_ElevatorCabin.Contract` (`local.Cabin`) false false)
      (elif (and (> _returnvalue_7 _returnvalue_2) (< _returnvalue_7 (+ _returnvalue_2 (`self.ContractOffsetDistance`))))
        (`/Game/PlaneContent/Blueprints/Systems/PlaneActors/Elevator/BP_ElevatorCabin.Contract` (`local.Cabin`) false true)))
    (elif (or (and (< _returnvalue_5 _returnvalue_4) (> _returnvalue_5 (- _returnvalue_4 (+ (`self.ContractOffsetDistance`) (`self.CabinHeight`))))) (and (> _returnvalue_6 _returnvalue) (< _returnvalue_6 (+ _returnvalue (`self.ContractOffsetDistance`)))))
      (`/Game/PlaneContent/Blueprints/Systems/PlaneActors/Elevator/BP_ElevatorCabin.Contract` (`local.Cabin`) true false))))

(fn `SpawnCabinsAlongSpline`
  (locals (CurrentSpawnDistance :type "Float (double-precision)") (DistanceBetweenCabins :type "Float (double-precision)" :default 50.0))
  (bind _returnvalue (`KismetMathLibrary.FFloor` (/ (`SplineComponent.GetSplineLength` (`self.Spline`)) (+ (`local.DistanceBetweenCabins`) (`self.CabinHeight`)))))
  (set `local.DistanceBetweenCabins` (+ (/ (`self.CabinHeight`) 2.0) 20.0))
  (set `local.DistanceBetweenCabins` (/ (- (`SplineComponent.GetSplineLength` (`self.Spline`)) (* (`self.CabinHeight`) _returnvalue)) _returnvalue))
  (for _ (range (+ _returnvalue 1))
    (bind _returnvalue_2 (`|SpawnActorFromClass` "/Game/PlaneContent/Blueprints/Systems/PlaneActors/Elevator/BP_ElevatorCabin.BP_ElevatorCabin_C" (`KismetMathLibrary.MakeTransform` (`SplineComponent.GetLocationAtDistanceAlongSpline` (`self.Spline`) (`local.CurrentSpawnDistance`) "World")) "Undefined" "MultiplyWithRoot" null null))
    (bind _returnvalue_3 (`KismetArrayLibrary.Array_Add` (`self.Cabins`) _returnvalue_2))
    (set `local.CurrentSpawnDistance` (+ (`local.CurrentSpawnDistance`) (+ (`local.DistanceBetweenCabins`) (`self.CabinHeight`))))
    (bind _returnvalue_4 (`SplineComponent.GetDistanceAlongSplineAtLocation` (`self.Spline`) (`self.K2_GetActorLocation` (`|GetArrayItem` (`self.Cabins`) _returnvalue_3)) "World"))
    (if (or (< _returnvalue_4 (+ (`SplineComponent.GetDistanceAlongSplineAtSplinePoint` (`self.Spline`) 1) (`self.RotateOffsetDistnace`))) (> _returnvalue_4 (+ (`SplineComponent.GetDistanceAlongSplineAtSplinePoint` (`self.Spline`) 3) (`self.RotateOffsetDistnace`))))
      (`/Game/PlaneContent/Blueprints/Systems/PlaneActors/Elevator/BP_ElevatorCabin.Rotate` (`|GetArrayItem` (`self.Cabins`) _returnvalue_3) true true))))

(fn `UserConstructionScript`
  (locals (InstancedSTatMeshArray :type "Array of InstancedStaticMeshComponent Object Reference"))
  (for (_array_element _array_index) _
    (`self.K2_SetActorLocationAndRotation` _array_element (`SplineComponent.GetLocationAtDistanceAlongSpline` (`self.Spline`) (* 0.0 _array_index) "Local") (`KismetMathLibrary.MakeRotator` 0.0) false false)))