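; Plane toilet actor that tracks occupancy, gets dirty after a set number of uses, and exposes door control plus wait and entry locations.
; Occupancy changes go through a server event, with multicasts updating the Free, Occupied or Dirty sign.
; Random line traces spawn attached stain actors, blocking occupancy changes only if the full dirt amount spawns.
; CheckIsClean resets the toilet once its stain list is empty.
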(event `self.ReceiveBeginPlay`
  (`self.SetIsOccupied` false true)
  (set `self.CurrentUses` 0))

(event `CheckIsClean`
  (bind _staininstances (`self.StainInstances`))
  (if (`KismetArrayLibrary.Array_IsEmpty` _staininstances)
    (`KismetSystemLibrary.PrintString` "Toilet is clean" true true (struct :`G` 1.0 :`B` 0.247149 :`A` 1.0) 5.0 "1")
    (`self.TryToSetDirty` false)
    (else
      (`KismetSystemLibrary.PrintString` (`KismetStringLibrary.Concat_StrStr` "Stans left: " (`KismetStringLibrary.Conv_IntToString` (`KismetArrayLibrary.Array_Length` _staininstances))) true true (struct :`R` 1.0 :`G` 0.736817 :`B` 0.371494 :`A` 1.0) 2.0 "1"))))

(event `Server_SetOccupied`
  (params (IsOccupied :type Boolean) (SetupAtStart :type Boolean))
  (if (not (`self.IsDirty`))
    (bind _output_get (set `self.IsOccupied` IsOccupied))
    (if _output_get
      (`self.Multicast_SetSign_Occupied`)
      (else
        (`self.Multicast_SetSign_Free`)
        (if (not SetupAtStart)
          (`/Engine/EditorBlueprintResources/StandardMacros.IncrementInt` (`self.CurrentUses`)
            (:`  `
              (if (== (`self.CurrentUses`) (`self.UsesAfterConsideredDirty`))
                (`self.TryToSetDirty` true)))))))))

(event `Multicast_SetSign_Free`
  (`PrimitiveComponent.SetMaterial` (`self.Sign`) 0 "/Game/PlaneContent/Debug/M_DebugColor_Good.M_DebugColor_Good")
  (`TextRenderComponent.K2_SetText` (`self.SignText`) "Free"))

(event `Multicast_SetSign_Occupied`
  (`KismetSystemLibrary.PrintString` "OCCUPIED" true true (struct :`R` 1.0 :`B` 0.568809 :`A` 1.0) 10.0)
  (`PrimitiveComponent.SetMaterial` (`self.Sign`) 0 "/Game/PlaneContent/Debug/M_DebugColor_Bad.M_DebugColor_Bad")
  (`TextRenderComponent.K2_SetText` (`self.SignText`) "Occupied"))

(event `Multicast_SetSign_Dirty`
  (`PrimitiveComponent.SetMaterial` (`self.Sign`) 0 "/Game/PlaneContent/Blueprints/Systems/PlaneActors/NeedActors/Toilet/M_ToiletDirtySign.M_ToiletDirtySign")
  (`TextRenderComponent.K2_SetText` (`self.SignText`) "Dirty"))

(fn `GetEntryLocation`
  (returns (EntryLocation :type "Vector Structure"))
  (return (`SceneComponent.K2_GetComponentLocation` (`self.EntryPoint`))))

(fn `GetWaitLocation`
  (returns (WaitLocation :type "Vector Structure"))
  (return (`SceneComponent.K2_GetComponentLocation` (`self.TargetPos`))))

(fn `OpenOrCloseDoor`
  (params (`Open?` :type Boolean))
  (returns (DoorAnimTime :type "Float (double-precision)"))
  (locals (AnimTime :type "Float (double-precision)" :default 1.0))
  (bind _asbp_physic_door (cast `/Game/PlaneContent/Blueprints/Systems/PlaneActors/PhysicDoor/BP_PhysicDoor` (`ChildActorComponent.ChildActor` (`self.BP_PhysicDoor`))))
  (`/Game/PlaneContent/Blueprints/Systems/PlaneActors/PhysicDoor/BP_PhysicDoor.StartDoorMovement` _asbp_physic_door `Open?`)
  (return (+ (`/Game/PlaneContent/Blueprints/Systems/PlaneActors/PhysicDoor/BP_PhysicDoor.OpenTime` _asbp_physic_door) 0.5)))

(fn `SetIsOccupied`
  (params (IsOccupied :type Boolean) (SetupAtStart :type Boolean))
  (locals (NewLocalVar :type Text :default "NSLOCTEXT(\"[B7F9C3F8973E01EECC1D01348C086965]\", \"440220D94F7EF36F451C1C94DCFA07E9\", \"Occupied\")") (NewLocalVar_0 :type Text :default "NSLOCTEXT(\"[B7F9C3F8973E01EECC1D01348C086965]\", \"D31F39C64F514814DE0F4EB0388016DE\", \"Free\")"))
  (`self.Server_SetOccupied` IsOccupied SetupAtStart))

(fn `SpawnDirt`
  (bind _returnvalue (`SceneComponent.K2_GetComponentLocation` (`self.DirtRaycastOrigin`)))
  (for _ (range (`self.DirtAmount`))
    (bind (_outhit _returnvalue_2) (`KismetSystemLibrary.LineTraceSingle` :`Start` _returnvalue :`End` (+ _returnvalue (* (`KismetMathLibrary.RandomUnitVector`) (`self.RaycastLength`))) :`TraceChannel` "TraceTypeQuery1" :`DrawDebugType` "ForDuration" :`bIgnoreSelf` false :`DrawTime` 10.0))
    (if _returnvalue_2
      (bind (_bblockinghit _binitialoverlap _time _distance _location _impactpoint _normal _impactnormal _physmat _hitactor _hitcomponent) (`GameplayStatics.BreakHitResult` _outhit))
      (bind _returnvalue_3 (`|SpawnActorFromClass` "/Game/PlaneContent/Blueprints/MiniGame/BP_Stains.BP_Stains_C" (`KismetMathLibrary.MakeTransform` _location (`KismetMathLibrary.FindLookAtRotation` _location (+ _location _normal))) "Undefined" "MultiplyWithRoot" null self null))
      (`KismetArrayLibrary.Array_Add` (`self.StainInstances`) _returnvalue_3)
      (`self.K2_AttachToComponent` _returnvalue_3 _hitcomponent "None" "KeepWorld" "KeepWorld" "KeepWorld" true)
      (else
        (`KismetSystemLibrary.PrintString` (`KismetStringLibrary.Concat_StrStr` "Toilet raycast for dirt decal spawning didn't collide (no dirt spawn and less dirt in total). Check Toilet area or increase raycast length. Toilet Actor: " (`KismetSystemLibrary.GetDisplayName` self)) true true (struct :`G` 0.66 :`B` 1.0 :`A` 1.0) 20.0))))
  (if (not (== (`self.DirtAmount`) (`KismetArrayLibrary.Array_Length` (`self.StainInstances`))))
    (`KismetSystemLibrary.PrintString` (`KismetStringLibrary.Concat_StrStr` "NOT ENOUGH DIRT WAS SPAWNED TO SET TOILET AS DIRTY (" (`KismetSystemLibrary.GetDisplayName` self) ")") true true (struct :`R` 1.0 :`A` 1.0) 20.0)
    (`KismetSystemLibrary.PrintString` (`KismetStringLibrary.Concat_StrStr` (`KismetStringLibrary.Conv_IntToString` (`self.DirtAmount`)) " //// " (`KismetStringLibrary.Conv_IntToString` (`KismetArrayLibrary.Array_Length` (`self.StainInstances`)))) true true (struct :`G` 0.66 :`B` 1.0 :`A` 1.0) 10.0)))

(fn `TryToSetDirty`
  (params (IsDirty :type Boolean))
  (locals (NewLocalVar_1 :type Text :default "NSLOCTEXT(\"[B7F9C3F8973E01EECC1D01348C086965]\", \"0943477646E4EE55822C38950670FE9B\", \"DIRTY\")"))
  (if IsDirty
    (`|ExecutionSequence`
      (:`then_0`
        (`self.SpawnDirt`)
        (if (== (`self.DirtAmount`) (`KismetArrayLibrary.Array_Length` (`self.StainInstances`)))
          (set `self.IsDirty` true)))
      (:`then_1`
        (`self.Multicast_SetSign_Dirty`)))
    (else
      (set `self.CurrentUses` 0)
      (set `self.IsDirty` false)
      (`self.SetIsOccupied` false))))

(fn `UserConstructionScript`)