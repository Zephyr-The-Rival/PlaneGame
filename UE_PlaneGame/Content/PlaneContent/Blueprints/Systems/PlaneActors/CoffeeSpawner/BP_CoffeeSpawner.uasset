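; BP_CoffeeSpawner is a spawner actor that keeps a replacement coffee cup (BP_Cup) coming at its own location.
; On BeginPlay it spawns the first cup if player character 0 has authority.
; SpawnCup skips near-zero locations, stores the new cup and binds to its OnEndPlay.
; SpawnNewCup handles a cup's end of play, clearing the reference and spawning another if the stored reference is still valid.
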(event `self.ReceiveBeginPlay`
  (if (`self.HasAuthority` (`GameplayStatics.GetPlayerCharacter` 0))
    (`self.SpawnCup` (`self.K2_GetActorLocation`))))

(event `SpawnNewCup`
  (params (Actor :type "Actor Object Reference") (EndPlayReason :type "EEndPlayReason Enum" :default "Destroyed"))
  (`/Engine/EditorBlueprintResources/StandardMacros.IsValid` (`self.CoffeeCups`)
    (:`Is Valid`
      (set `self.CoffeeCups` null)
      (`self.SpawnCup` (`self.K2_GetActorLocation`)))))

(fn `SpawnCup`
  (params (SpawnLocation :type "Vector Structure"))
  (if (!= SpawnLocation (0.0 0.0 0.0) :`ErrorTolerance` 0.1)
    (bind _returnvalue (`|SpawnActorFromClass` "/Game/PlaneContent/Blueprints/Items/BP_Cup.BP_Cup_C" (`KismetMathLibrary.MakeTransform` SpawnLocation) "Undefined" "MultiplyWithRoot" null null))
    (set `self.CoffeeCups` _returnvalue)
    (add `self.OnEndPlay` _returnvalue (`|CreateDelegate` :!event `SpawnNewCup`))))

(fn `UserConstructionScript`)