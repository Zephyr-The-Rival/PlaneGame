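; Physics door that players pull by its handle, with a scripted open/close movement intended mainly for NPC State Trees.
; Grabbing enables physics and tracks hands; each tick, a debug-drawn impulse at the handle pulls toward their summed direction.
; A repeat grab removes that hand, and the last removal disables physics and closes the door.
; Scripted movement runs a yaw Timeline, resumed from the current angle, only while physics is off.
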(event `self.ReceiveBeginPlay`
  (`PrimitiveComponent.SetSimulatePhysics` (`self.Door`) false))

(event `self.ReceiveTick`
  (params (DeltaSeconds :type "Float (single-precision)"))
  (`|ExecutionSequence`
    (:`then_0`
      (`self.ApplyForceAtDoorToPlayer`))))

(event `StartDoorMovement`
  (params (Open :type Boolean))
  (bind (_returnvalue_roll _returnvalue_pitch _returnvalue_yaw) (`KismetMathLibrary.BreakRotator` (`SceneComponent.K2_GetComponentRotation` (`self.Door`))))
  (bind (_returnvalue_roll_2 _returnvalue_pitch_2 _returnvalue_yaw_2) (`KismetMathLibrary.BreakRotator` (`SceneComponent.K2_GetComponentRotation` (`self.DefaultSceneRoot`))))
  (bind (_returnvalue_roll_3 _returnvalue_pitch_3 _returnvalue_yaw_3) (`KismetMathLibrary.BreakRotator` (`SceneComponent.K2_GetComponentRotation` (`self.DefaultSceneRoot`))))
  (bind (_returnvalue_roll_4 _returnvalue_pitch_4 _returnvalue_yaw_4) (`KismetMathLibrary.BreakRotator` (`SceneComponent.K2_GetComponentRotation` (`self.Door`))))
  (bind (_returnvalue_roll_5 _returnvalue_pitch_5 _returnvalue_yaw_5) (`KismetMathLibrary.BreakRotator` (`SceneComponent.K2_GetComponentRotation` (`self.DefaultSceneRoot`))))
  (bind _returnvalue (`KismetMathLibrary.Abs` (- (+ (+ _returnvalue_yaw_4 180.0) 360.0) (+ (+ _returnvalue_yaw_3 180.0) 360.0))))
  (bind _returnvalue_2 (/ (`KismetMathLibrary.SelectFloat` (- 360.0 _returnvalue) _returnvalue (>= _returnvalue 180.0)) (`self.OpenAngle`)))
  ; Fixed Door movement (no physics) // Mainly for npcs state tree
  (if (not (`SceneComponent.IsSimulatingPhysics` (`self.Door`) "None"))
    (`TimelineComponent.SetPlayRate` (`self.Timeline`) (/ 1.0 (`self.OpenTime`)))
    (`|ExecutionSequence`
      (:`then_0`
        (if (and (!= _returnvalue_yaw _returnvalue_yaw_2) (!= _returnvalue_yaw (+ _returnvalue_yaw_2 (`self.OpenAngle`))))
          (bind (_direction _newtrack_0) (`Timeline|Timeline` :`NewTime` (`KismetMathLibrary.SelectFloat` (- 1.0 _returnvalue_2) _returnvalue_2 Open) :!via `SetNewTime` :!label _label)
            (:`Update`
              (`SceneComponent.K2_SetWorldRotation` (`self.Door`) (`KismetMathLibrary.MakeRotator` 0.0 0.0 (`KismetMathLibrary.Lerp` _returnvalue_yaw_5 (+ _returnvalue_yaw_5 (`self.OpenAngle`)) _newtrack_0)) false false)))))
      (:`then_1`
        (if Open
          (goto _label)
          (else
            (goto _label :!via `Reverse`)))))))

(event `self.OnHandReleased`
  (params (Hand :type "PlayerHand Object Reference") (PlayerCharacter :type "PlanePlayerCharacter Object Reference"))
  ; Why does this not get triggered in the c++ code?
  (if (`KismetArrayLibrary.Array_Contains` (`self.Hands`) Hand)
    _))

(event `self.OnHandGrabbed`
  (params (Hand :type "PlayerHand Object Reference") (PlayerCharacter :type "PlanePlayerCharacter Object Reference"))
  ; Handle Grab Handle
  (`PrimitiveComponent.SetSimulatePhysics` (`self.Door`) true)
  (if (`KismetArrayLibrary.Array_Contains` (`self.Hands`) Hand)
    (`KismetArrayLibrary.Array_RemoveItem` (`self.Hands`) Hand)
    (`KismetArrayLibrary.Array_RemoveItem` (`self.Player`) PlayerCharacter)
    (if (`KismetArrayLibrary.Array_IsEmpty` (`self.Hands`))
      (`PrimitiveComponent.SetSimulatePhysics` (`self.Door`) false)
      (set `self.ApplyForce` false)
      (`self.StartDoorMovement` false))
    (else
      (`KismetArrayLibrary.Array_Add` (`self.Hands`) Hand)
      (`KismetArrayLibrary.Array_Add` (`self.Player`) PlayerCharacter)
      (set `self.ApplyForce` true))))

(event `ApplyForceAtDoorToPlayer`
  (bind _returnvalue (`SceneComponent.K2_GetComponentLocation` (`self.BP_GrabHandle`)))
  (bind _returnvalue_2 (* (`KismetMathLibrary.Normal` (`self.ForceVector`)) (`self.Force`)))
  ; Handle Grab Handle
  ;;[0.007264 0.03556 0.15 0.5] Handle Force during grabbing
  (if (`self.ApplyForce`)
    (set `self.ForceVector` (0.0 0.0 0.0))
    (for (_ _array_index) (`self.Hands`)
      (set `self.ForceVector` (+ (`self.ForceVector`) (- (`self.K2_GetActorLocation` (`ChildActorComponent.ChildActor` (`PlanePlayerCharacter.PlayerHandCA` (`|GetArrayItem` (`self.Player`) _array_index)))) (`SceneComponent.K2_GetComponentLocation` (`self.BP_GrabHandle`))))))
    (`PrimitiveComponent.AddImpulseAtLocation` (`self.Door`) _returnvalue_2 _returnvalue "None")
    (`KismetSystemLibrary.DrawDebugLine` _returnvalue (+ _returnvalue _returnvalue_2) (struct :`G` 0.295438 :`B` 1.0 :`A` 1.0) 0.1 1.0)))

(fn `UserConstructionScript`)