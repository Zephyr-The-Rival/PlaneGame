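; Passenger component that simulates needs from the owner's personality and feeds them into satisfaction.
; A looping timer raises each need's demand by its multiplier, promoting one past its threshold to current when none is active.
; Past its anger threshold, the current need starts a timer draining satisfaction; at expiry it applies a penalty and resets to random demand.
; Fulfillment logic is unconnected.
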(event `self.ReceiveBeginPlay`
  (`self.Init`)
  (`KismetSystemLibrary.Delay` 0.2)
  (`self.FillNeeds`)
  (`KismetSystemLibrary.K2_SetTimerDelegate` (`|CreateDelegate` :!event `UpdateNeeds`) (`self.NeedsTick`) true))

(event `UpdateNeeds`
  (set `self.PossibleNeed` (struct))
  (for (_array_element _array_index) (`self.Needs`)
    (`self.IncreaseNeedByPersonality` _array_index)
    (`self.CheckForPossibleNeed` _array_element)
    (`self.CheckForNeedToExpire`))
  (`self.SetCurrentNeedIfValid`))

(event `TryToFullfillCurrentNeed`)

(event `StartAngryTick`
  ; Angry Tick
  (if (not (`KismetSystemLibrary.K2_IsValidTimerHandle` (`self.AngryTimerHandle`)))
    (bind _returnvalue (`KismetSystemLibrary.K2_SetTimerDelegate` (`|CreateDelegate` :!event `AngryTick`) (`self.NeedsTick`) true))
    (set `self.AngryTimerHandle` _returnvalue)))

(event `StopAngryTick`
  ; Angry Tick
  (`KismetSystemLibrary.K2_ClearAndInvalidateTimerHandle` (`self.AngryTimerHandle`)))

(event `NeedExpired`
  (`|ExecutionSequence`
    (:`then_0`
      ; Lower satisfaction in pawn
      (bind (_currentdemand _multiplier _demandthreshold _angrythreshold _success) (`self.GetCurrentNeedValues`))
      (if _success
        (`/Game/PlaneContent/Blueprints/Systems/Passenger/BP_Passenger.AdjustSatisfaction` (`self.Passenger`) _multiplier true false)
        (`self.ResetCurrentNeed`)))
    (:`then_1`
      (`self.OnNeedExpired`))))

(fn `AngryTick`
  (bind (_currentdemand _multiplier _demandthreshold _angrythreshold _success) (`self.GetCurrentNeedValues`))
  (if _success
    (`/Game/PlaneContent/Blueprints/Systems/Passenger/BP_Passenger.AdjustSatisfaction` (`self.Passenger`) _multiplier true true)))

(fn `CheckForNeedToExpire`
  (if (not (`self.HasNoCurrentNeed`))
    (for _array_element (`self.Needs`)
      (bind (_need _currentdemand) (break `/Game/PlaneContent/Blueprints/Systems/Passenger/Components/Needs/ST_Need` _array_element))
      (if (and (`|EnumEquality` (`self.CurrentNeed`) _need) (>= _currentdemand (`self.ExpireThreshold`)))
        (`|ExecutionSequence`
          (:`then_0`
            (`self.NeedExpired`))
          (:`then_1`
            (break)))
        (else
          (bind (_need_2 _currentdemand_2 _multiplier _demandthreshold _angrythreshold) (break `/Game/PlaneContent/Blueprints/Systems/Passenger/Components/Needs/ST_Need` _array_element))
          (if (and (`|EnumEquality` (`self.CurrentNeed`) _need_2) (>= _currentdemand_2 _angrythreshold))
            (`|ExecutionSequence`
              (:`then_0`
                (`self.StartAngryTick`))
              (:`then_1`
                (break)))))))))

(fn `CheckForPossibleNeed`
  (params (Need :type "/Game/PlaneContent/Blueprints/Systems/Passenger/Components/Needs/ST_Need Structure (by ref)"))
  (bind (_need _currentdemand) (break `/Game/PlaneContent/Blueprints/Systems/Passenger/Components/Needs/ST_Need` Need))
  (bind ((`CurrentDemand_9_67B552EA4140F375FC1079ABB6C05EBB` _currentdemand_2) (`DemandThreshold_10_1A912EEA4C07CEE6DCCA64BA857DF93E` _demandthreshold)) (break `/Game/PlaneContent/Blueprints/Systems/Passenger/Components/Needs/ST_Need` Need))
  (if (and (`self.HasNoCurrentNeed`) (>= _currentdemand_2 _demandthreshold))
    (if (> _currentdemand (`.CurrentDemand_9_67B552EA4140F375FC1079ABB6C05EBB` (break `/Game/PlaneContent/Blueprints/Systems/Passenger/Components/Needs/ST_Need` (`self.PossibleNeed`))))
      (set `self.PossibleNeed` (make `/Game/PlaneContent/Blueprints/Systems/Passenger/Components/Needs/ST_Need` _need)))))

(fn `FillNeeds`
  (`KismetArrayLibrary.Array_Clear` (`self.Needs`))
  (for _array_element (`/Game/PlaneContent/Blueprints/Systems/Passenger/Components/Personality/AC_Personality.NeedBehaviors` (`self.Personality`))
    (bind (_need _multiplier _demandthreshold _angrythreshold) (break `/Game/PlaneContent/Blueprints/Systems/Passenger/Components/Personality/ST_NeedBehavior` _array_element))
    (if (`|EnumInequality` _need "NewEnumerator6")
      (`KismetArrayLibrary.Array_Add` (`self.Needs`) (make `/Game/PlaneContent/Blueprints/Systems/Passenger/Components/Needs/ST_Need` _need (`self.GetRandomDemand`) _multiplier _demandthreshold _angrythreshold))))
  (set `self.CurrentNeed` "NewEnumerator6"))

(fn `GetCurrentNeedValues`
  (returns (CurrentDemand :type "Float (double-precision)") (Multiplier :type "Float (double-precision)") (DemandThreshold :type "Float (double-precision)") (AngryThreshold :type "Float (double-precision)") (Success :type Boolean))
  (bind (_success _structrefindex) (`self.GetNeedStructIndex` (`self.CurrentNeed`)))
  (if _success
    (bind ((`CurrentDemand_9_67B552EA4140F375FC1079ABB6C05EBB` _currentdemand) (`Multiplier_15_2463CFC84F15FB129E95C5BDA3440D95` _multiplier) (`DemandThreshold_10_1A912EEA4C07CEE6DCCA64BA857DF93E` _demandthreshold) (`AngryThreshold_13_8956BFB14A4291F18D9CA2AEC1AEF044` _angrythreshold)) (break `/Game/PlaneContent/Blueprints/Systems/Passenger/Components/Needs/ST_Need` (`|GetArrayItem` (`self.Needs`) _structrefindex)))
    (return _currentdemand _multiplier _demandthreshold _angrythreshold true)
    (else
      (return 0.0 0.0 0.0 0.0 false))))

(fn `GetNeedStructIndex`
  (params (Need :type "/Game/PlaneContent/Blueprints/Systems/Passenger/Components/Needs/Enum_PassengerNeeds Enum" :default "NewEnumerator6"))
  (returns (Success :type Boolean) (StructRefIndex :type Integer))
  (locals (ReturnIndex :type Integer :default -1))
  (for (_array_element _array_index) (`self.Needs`)
    (if (`|EnumEquality` Need (`.Need_5_E5623B3D4840392DC8B41B9FE6FB0224` (break `/Game/PlaneContent/Blueprints/Systems/Passenger/Components/Needs/ST_Need` _array_element)))
      (set `local.ReturnIndex` _array_index)
      (break)))
  (if (>= (`local.ReturnIndex`) 0)
    (return true (`local.ReturnIndex`))
    (else
      (return false -1))))

(fn `GetPersonality`
  (bind _returnvalue (`self.GetOwner`))
  (bind _asbp_passenger (cast `/Game/PlaneContent/Blueprints/Systems/Passenger/BP_Passenger` _returnvalue)
    (:`then`
      (set `self.Personality` (`/Game/PlaneContent/Blueprints/Systems/Passenger/BP_Passenger.AC_Personality` _asbp_passenger)))
    (:`CastFailed`
      (`KismetSystemLibrary.PrintString` (`KismetStringLibrary.Concat_StrStr` "No Personality Component in passenger " "(" (`KismetSystemLibrary.GetDisplayName` _returnvalue) ")") true true (struct :`R` 1.0 :`A` 1.0) 10.0))))

(fn `IncreaseNeedByPersonality`
  (params (Index :type Integer))
  (bind _output (`|GetArrayItem` (`self.Needs`) Index))
  (bind ((`CurrentDemand_9_67B552EA4140F375FC1079ABB6C05EBB` _currentdemand) (`Multiplier_15_2463CFC84F15FB129E95C5BDA3440D95` _multiplier)) (break `/Game/PlaneContent/Blueprints/Systems/Passenger/Components/Needs/ST_Need` _output))
  (setmembers `/Game/PlaneContent/Blueprints/Systems/Passenger/Components/Needs/ST_Need` :`StructRef` _output :`CurrentDemand` (+ _currentdemand (* _multiplier (`self.NeedIncrease`)))))

(fn `Init`
  (`|ExecutionSequence`
    (:`then_0`
      (bind _asbp_passenger (cast `/Game/PlaneContent/Blueprints/Systems/Passenger/BP_Passenger` (`self.GetOwner`)))
      (set `self.Passenger` _asbp_passenger))
    (:`then_1`
      (`self.GetPersonality`))))

(fn `ResetCurrentNeed`
  (bind (_success _structrefindex) (`self.GetNeedStructIndex` (`self.CurrentNeed`)))
  (if _success
    (setmembers `/Game/PlaneContent/Blueprints/Systems/Passenger/Components/Needs/ST_Need` :`StructRef` (`|GetArrayItem` (`self.Needs`) _structrefindex) :`CurrentDemand` (`self.GetRandomDemand`))
    (set `self.CurrentNeed` "NewEnumerator6")
    (`self.StopAngryTick`)))

(fn `SetCurrentNeedIfValid`
  (if (and (`self.HasNoCurrentNeed`) (`|EnumInequality` (`.Need_5_E5623B3D4840392DC8B41B9FE6FB0224` (break `/Game/PlaneContent/Blueprints/Systems/Passenger/Components/Needs/ST_Need` (`self.PossibleNeed`))) "NewEnumerator6"))
    (set `self.CurrentNeed` (`.Need_5_E5623B3D4840392DC8B41B9FE6FB0224` (break `/Game/PlaneContent/Blueprints/Systems/Passenger/Components/Needs/ST_Need` (`self.PossibleNeed`))))
    (`self.OnNewNeedAppreared`)))