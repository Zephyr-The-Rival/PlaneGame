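; Passenger speech component that shows speech bubbles above a BP_Passenger for needs and reactions.
; On the server, it binds to AC_PassengerNeeds events, spawning a need bubble for new needs and brief smile or curse bubbles on fulfillment or expiry.
; A looping timer shows a curse bubble when satisfaction is low and no bubble exists.
; Each new bubble replaces the current one; delayed deletion only removes non-need bubbles.
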(event `self.ReceiveBeginPlay`
  (if (`Actor.HasAuthority` (`self.GetOwner`))
    (`self.Init`)
    (`self.SubscribeToNeedComponent`)
    (bind _returnvalue (`KismetSystemLibrary.K2_SetTimerDelegate` (`|CreateDelegate` :!event `SpeechTick`) 5.0 true))
    (set `self.SpeechTickTimer` _returnvalue)))

(event `OnNewNeedAppeared`
  (params (Need :type "/Game/PlaneContent/Blueprints/Systems/Passenger/Components/Needs/Enum_PassengerNeeds Enum" :default "NewEnumerator6"))
  (`self.SpawnNeedSpeechBubble` Need))

(event `OnNeedFullfilled`
  (`self.SpawnNoneNeedSpeechBubble` (`self.SmileSprite`))
  (`self.DeleteNoneSpeechBubbleWithDelay` 2.0))

(event `OnNeedExpired`
  (`self.SpawnNoneNeedSpeechBubble` (`self.CurseSprite`))
  (`self.DeleteNoneSpeechBubbleWithDelay` 2.0))

(event `SpeechTick`
  (bind _passenger (`self.Passenger`))
  (`/Engine/EditorBlueprintResources/StandardMacros.IsValid` (`self.CurrentSpeechBubble`)
    (:`Is Not Valid`
      (`|ExecutionSequence`
        (:`then_0`
          (`/Engine/EditorBlueprintResources/StandardMacros.IsValid` _passenger
            (:`Is Valid`
              (if (< (`/Game/PlaneContent/Blueprints/Systems/Passenger/BP_Passenger.Satisfaction` _passenger) -10.0)
                (`self.SpawnNoneNeedSpeechBubble` (`self.CurseSprite`))
                (`self.DeleteNoneSpeechBubbleWithDelay` 5.0)))))))))

(event `DeleteNoneSpeechBubbleWithDelay`
  (params (Duration :type "Float (single-precision)"))
  (bind _currentspeechbubble (`self.CurrentSpeechBubble`))
  (`KismetSystemLibrary.Delay` Duration)
  (`/Engine/EditorBlueprintResources/StandardMacros.IsValid` _currentspeechbubble
    (:`Is Valid`
      (if (`|EnumEquality` (`/Game/PlaneContent/Blueprints/Systems/Passenger/Components/Speech/BP_SpeechBubble.Need` _currentspeechbubble) "NewEnumerator6")
        (`Actor.K2_DestroyActor` (`self.CurrentSpeechBubble`))))))

(fn `Init`
  (bind _returnvalue (`self.GetOwner`))
  (bind _returnvalue_2 (`Actor.GetComponentByClass` _returnvalue "/Game/PlaneContent/Blueprints/Systems/Passenger/Components/Needs/AC_PassengerNeeds.AC_PassengerNeeds_C"))
  (`|ExecutionSequence`
    (:`then_0`
      (`/Engine/EditorBlueprintResources/StandardMacros.IsValid` _returnvalue_2
        (:`Is Valid`
          (set `self.NeedComponent` _returnvalue_2))
        (:`Is Not Valid`
          (`KismetSystemLibrary.PrintString` (`KismetStringLibrary.Concat_StrStr` "NO PASSENGER NEEDS COMPONENT FOUND!!!" "(" (`KismetSystemLibrary.GetDisplayName` _returnvalue) ")") true true (struct :`R` 1.0 :`A` 1.0) 10.0))))
    (:`then_1`
      (bind _asbp_passenger (cast `/Game/PlaneContent/Blueprints/Systems/Passenger/BP_Passenger` (`self.GetOwner`)))
      (set `self.Passenger` _asbp_passenger))))

(fn `SpawnNeedSpeechBubble`
  (params (Need :type "/Game/PlaneContent/Blueprints/Systems/Passenger/Components/Needs/Enum_PassengerNeeds Enum" :default "NewEnumerator6"))
  (if (`Actor.HasAuthority` (`self.GetOwner`))
    (bind _currentspeechbubble (`self.CurrentSpeechBubble`)
      (:`then`
        (`Actor.K2_DestroyActor` _currentspeechbubble))
      (:`else`
        _))
    (bind _asbp_passenger (cast `/Game/PlaneContent/Blueprints/Systems/Passenger/BP_Passenger` (`self.GetOwner`)))
    (bind _returnvalue (`|SpawnActorFromClass` "/Game/PlaneContent/Blueprints/Systems/Passenger/Components/Speech/BP_SpeechBubble.BP_SpeechBubble_C" (`KismetMathLibrary.MakeTransform` (+ (0.0 0.0 0.0) (`KismetMathLibrary.MakeVector` 0.0 0.0 (+ (`CapsuleComponent.GetUnscaledCapsuleHalfHeight` (`Character.CapsuleComponent` _asbp_passenger)) 10.0)))) "Undefined" "MultiplyWithRoot" null _asbp_passenger))
    (set `/Game/PlaneContent/Blueprints/Systems/Passenger/Components/Speech/BP_SpeechBubble.Need` (`local.Need`) _returnvalue)
    (bind _output_get (set `self.CurrentSpeechBubble` _returnvalue))
    (`Actor.K2_AttachToActor` _output_get _asbp_passenger "None" "KeepRelative" "KeepRelative" "KeepRelative" true)
    (set `/Game/PlaneContent/Blueprints/Systems/Passenger/Components/Speech/BP_SpeechBubble.NeedComponent` (`self.NeedComponent`) _output_get)))

(fn `SpawnNoneNeedSpeechBubble`
  (params (Sprite :type "PaperSprite Object Reference"))
  (if (`Actor.HasAuthority` (`self.GetOwner`))
    (bind _currentspeechbubble (`self.CurrentSpeechBubble`)
      (:`then`
        (`Actor.K2_DestroyActor` _currentspeechbubble))
      (:`else`
        _))
    (bind _asbp_passenger (cast `/Game/PlaneContent/Blueprints/Systems/Passenger/BP_Passenger` (`self.GetOwner`)))
    (bind _returnvalue (`|SpawnActorFromClass` "/Game/PlaneContent/Blueprints/Systems/Passenger/Components/Speech/BP_SpeechBubble.BP_SpeechBubble_C" (`KismetMathLibrary.MakeTransform` (+ (0.0 0.0 0.0) (`KismetMathLibrary.MakeVector` 0.0 0.0 (+ (`CapsuleComponent.GetUnscaledCapsuleHalfHeight` (`Character.CapsuleComponent` _asbp_passenger)) 10.0)))) "Undefined" "MultiplyWithRoot" null _asbp_passenger))
    (set `/Game/PlaneContent/Blueprints/Systems/Passenger/Components/Speech/BP_SpeechBubble.Need` "NewEnumerator6" _returnvalue)
    (set `/Game/PlaneContent/Blueprints/Systems/Passenger/Components/Speech/BP_SpeechBubble.Sprite` (`local.Sprite`) _returnvalue)
    (bind _output_get (set `self.CurrentSpeechBubble` _returnvalue))
    (`Actor.K2_AttachToActor` _output_get _asbp_passenger "None" "KeepRelative" "KeepRelative" "KeepRelative" true)
    (set `/Game/PlaneContent/Blueprints/Systems/Passenger/Components/Speech/BP_SpeechBubble.NeedComponent` (`self.NeedComponent`) _output_get)))

(fn `SubscribeToNeedComponent`
  (bind _needcomponent (`self.NeedComponent`)
    (:`then`
      (add `/Game/PlaneContent/Blueprints/Systems/Passenger/Components/Needs/AC_PassengerNeeds.OnNeedFullfilled` _needcomponent (`|CreateDelegate` :!event `OnNeedFullfilled`))
      (add `/Game/PlaneContent/Blueprints/Systems/Passenger/Components/Needs/AC_PassengerNeeds.OnNeedExpired` _needcomponent (`|CreateDelegate` :!event `OnNeedExpired`))
      (add `/Game/PlaneContent/Blueprints/Systems/Passenger/Components/Needs/AC_PassengerNeeds.OnNewNeedAppreared` _needcomponent (`|CreateDelegate` :!event `ONNewNeedAppeared`)))
    (:`else`)))