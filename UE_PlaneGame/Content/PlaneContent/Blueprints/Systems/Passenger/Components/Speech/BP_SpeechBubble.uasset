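; Speech bubble actor in the passenger system that displays an icon for a passenger's need.
; On BeginPlay it looks up the sprite matching its Need in NeedSprites and applies it to both icon components.
; Every tick it rotates its root on yaw only to face the player pawn.
; An unfinished bubble color adjustment based on the NeedComponent's demand and anger threshold exists but never runs.
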(event `self.ReceiveBeginPlay`
  (`self.Init`))

(event `self.ReceiveTick`
  (params (DeltaSeconds :type "Float (single-precision)"))
  (`|ExecutionSequence`
    (:`then_0`
      (`self.FacePlayer`))
    (:`then_1`)))

(fn `AdjustBubbleDisplay`
  (locals (DemandAboveDemandThreshold :type "Float (double-precision)"))
  (bind _needcomponent (`self.NeedComponent`)
    (:`then`
      (bind (_currentdemand _multiplier _demandthreshold _angrythreshold _success) (`/Game/PlaneContent/Blueprints/Systems/Passenger/Components/Needs/AC_PassengerNeeds.GetCurrentNeedValues` _needcomponent))
      (if _success
        (set `local.DemandAboveDemandThreshold` (- _currentdemand _demandthreshold))
        (if (< _currentdemand _angrythreshold)
          ; Not angry yet
          (`PaperSpriteComponent.SetSpriteColor` :`self` (`self.SpeechBubble`)))))
    (:`else`)))

(fn `FacePlayer`
  (bind (_returnvalue_roll _returnvalue_pitch _returnvalue_yaw) (`KismetMathLibrary.BreakRotator` (`KismetMathLibrary.FindLookAtRotation` (`self.K2_GetActorLocation` self) (`self.K2_GetActorLocation` (`GameplayStatics.GetPlayerPawn` 0)))))
  (`SceneComponent.K2_SetWorldRotation` (`self.DefaultSceneRoot`) (`KismetMathLibrary.MakeRotator` 0.0 0.0 _returnvalue_yaw) false false))

(fn `Init`
  (for _array_element (`self.NeedSprites`)
    (bind (_need _sprite) (break `/Game/PlaneContent/Blueprints/Systems/Passenger/Components/Speech/ST_NeedIcons` _array_element))
    (if (`|EnumEquality` _need (`self.Need`))
      (`PaperSpriteComponent.SetSprite` (`self.NeedIcon`) _sprite)
      (`PaperSpriteComponent.SetSprite` (`self.NeedIcon1`) _sprite))))

(fn `UserConstructionScript`)