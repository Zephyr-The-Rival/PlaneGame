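; Passenger personality component that defines how a passenger's needs behave.
; On BeginPlay it reads every row of its personality DataTable and builds a NeedBehaviors collection of need, multiplier, demand threshold and anger threshold, skipping one sentinel need type.
; If no valid table is assigned, it prints a red on-screen error naming the owning passenger.
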(event `self.ReceiveBeginPlay`
  (`self.FillNeedBehaviors`))

(fn `FillNeedBehaviors`
  (bind _personalitytable (`self.PersonalityTable`))
  (`/Engine/EditorBlueprintResources/StandardMacros.IsValid` _personalitytable
    (:`Is Valid`
      (bind _outrownames (`DataTableFunctionLibrary.GetDataTableRowNames` _personalitytable))
      (for _array_element _outrownames
        (bind _returnvalue (`|GetDataTableRow` _personalitytable _array_element)
          (:`then`
            (bind (_need _multiplier _demandthreshold _angrythreshold) (break `/Game/PlaneContent/Blueprints/Systems/Passenger/Components/Personality/ST_NeedBehavior` _returnvalue))
            (if (`|EnumInequality` _need "NewEnumerator6")
              (`KismetArrayLibrary.Array_Add` (`self.NeedBehaviors`) (make `/Game/PlaneContent/Blueprints/Systems/Passenger/Components/Personality/ST_NeedBehavior` _need _multiplier _demandthreshold _angrythreshold)))))))
    (:`Is Not Valid`
      (`KismetSystemLibrary.PrintString` (`KismetStringLibrary.Concat_StrStr` "No Personality Component in passenger " "(" (`KismetSystemLibrary.GetDisplayName` (`self.GetOwner`)) ")") true true (struct :`R` 1.0 :`A` 1.0) 10.0))))