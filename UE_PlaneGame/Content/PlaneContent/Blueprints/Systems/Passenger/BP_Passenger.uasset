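; BP_Passenger is an airplane passenger that occupies an assigned seat and tracks a satisfaction score.
; TakeSeat snaps it to the transform of the seat stored by SetSeatAndRow and marks that seat occupied on its row.
; AdjustSatisfaction raises or lowers satisfaction by a tick or fulfillment amount scaled by a need multiplier, then broadcasts the change.
; A seat index check exists, but TakeSeat's branch is hardwired true.
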(fn `AdjustSatisfaction`
  (params (NeedMultiplier :type "Float (double-precision)") (LowerSatisfaction :type Boolean) (`SatisfactionTick?` :type Boolean))
  (set `self.Satisfaction` (+ (* (`KismetMathLibrary.SelectFloat` (`KismetMathLibrary.SelectFloat` (* (`self.SatisfactionOverTime`) -1.0) (`self.SatisfactionOverTime`) (`local.LowerSatisfaction`)) (`KismetMathLibrary.SelectFloat` (* (`self.FullfillIncrease`) -1.0) (`self.FullfillIncrease`) (`local.LowerSatisfaction`)) (`local.SatisfactionTick?`)) (`local.NeedMultiplier`)) (`self.Satisfaction`)))
  (`self.OnSatisfactionChanged` (`self.Satisfaction`)))

(fn `CheckForValidSeatIndex`
  (returns (ReturnValue :type Boolean))
  (return (not (or (< (`self.AssignedSeatIndex`) 0) (> (- (`self.AssignedSeatIndex`) 1) (`KismetArrayLibrary.Array_Length` (`/Game/PlaneContent/Blueprints/Systems/PlaneActors/SeatRows/Base/ActorPassengerSeatRow.PassengerSeats` (`self.AssignedSeatRow`))))))))

(fn `SetSeatAndRow`
  (params (SeatIndex :type Integer) (SeatRow :type "/Game/PlaneContent/Blueprints/Systems/PlaneActors/SeatRows/Base/ActorPassengerSeatRow Object Reference"))
  (set `self.AssignedSeatIndex` SeatIndex)
  (set `self.AssignedSeatRow` SeatRow))

(fn `TakeSeat`
  (bind _output (`|GetArrayItem` (`/Game/PlaneContent/Blueprints/Systems/PlaneActors/SeatRows/Base/ActorPassengerSeatRow.PassengerSeats` (`self.AssignedSeatRow`)) (`self.AssignedSeatIndex`)))
  (if true
    (`self.K2_SetActorLocation` (`self.K2_GetActorLocation` _output))
    (`self.K2_SetActorRotation` (`self.K2_GetActorRotation` _output))
    (`/Game/PlaneContent/Blueprints/Systems/PlaneActors/SeatRows/Base/ActorPassengerSeatRow.SetSeatOccupied` (`self.AssignedSeatRow`) true (`self.AssignedSeatIndex`))
    (else
      (`KismetSystemLibrary.PrintString` (`KismetStringLibrary.Concat_StrStr` "No valid Seat: " (`KismetSystemLibrary.GetDisplayName` self))))))

(fn `UserConstructionScript`)