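; BP_WorldButton is an interactable world button that animates its press when a player interacts with it.
; Server-side overrides of Interact, HoldInteractStart and HoldInteractEnd call the parent logic, then fire multicast events so all clients see the movement.
; Separate timelines drive the Button component's relative Z: a full press for single taps, and down and up halves for holds.
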(event `self.Interact`
  (params (InteractingPlayer :type "PlanePlayerCharacter Object Reference"))
  ; SinglePress
  (`parent.Interact` InteractingPlayer)
  (`self.Multicast_MoveButton`))

(event `self.HoldInteract_Start`
  (params (InteractingPlayer :type "PlanePlayerCharacter Object Reference"))
  (`parent.HoldInteract_Start` InteractingPlayer)
  (`self.Multicast_ButtonDown`))

(event `self.HoldInteract_End`
  (params (InteractingPlayer :type "PlanePlayerCharacter Object Reference"))
  (`parent.HoldInteract_End` InteractingPlayer)
  (`self.Mulitcast_ButtonUp`))

(event `Multicast_MoveButton`
  ; SinglePress
  (bind (_direction _0_1_0) (`Timeline|ButtonPressTL` :!via `PlayFromStart`)
    (:`Update`
      (`SceneComponent.K2_SetRelativeLocation` (`self.Button`) (`KismetMathLibrary.MakeVector` 0.0 0.0 (* _0_1_0 -5.0)) false false))))

(event `Multicast_ButtonDown`
  (bind (_direction _0_1) (`Timeline|ButtonDownTl` :!via `PlayFromStart`)
    (:`Update`
      (`SceneComponent.K2_SetRelativeLocation` (`self.Button`) (`KismetMathLibrary.MakeVector` 0.0 0.0 (* _0_1 -5.0)) false false))))

(event `Mulitcast_ButtonUp`
  (bind (_direction _1_0) (`Timeline|ButtonUP_TL` :!via `PlayFromStart`)
    (:`Update`
      (`SceneComponent.K2_SetRelativeLocation` (`self.Button`) (`KismetMathLibrary.MakeVector` 0.0 0.0 (* _1_0 -5.0)) false false))))

(fn `UserConstructionScript`)