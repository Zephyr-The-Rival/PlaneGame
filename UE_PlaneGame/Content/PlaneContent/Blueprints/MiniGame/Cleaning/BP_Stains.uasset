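; BP_Stains is a cleanable decal stain for the cleaning minigame, faded by repeated cleaning hits.
; CleanStain lowers Dirtiness on the authority, which drives the opacity of a dynamic decal material created at BeginPlay.
; Near zero dirtiness, the stain removes itself from its ToiletActor, triggers that actor's clean check and is destroyed.
; RepNotify variables sync opacity and the attached decal's transform to clients.
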(event `self.ReceiveBeginPlay`
  (bind _decal (`self.Decal`))
  (`|ExecutionSequence`
    (:`then_0`
      ; Set transform on client after attaching decals to hit object
      (if (`self.HasAuthority` (`GameplayStatics.GetPlayerCharacter` 0))
        (set `self.Transform` (`self.GetTransform`))))
    (:`then_1`
      (bind _returnvalue (`DecalComponent.CreateDynamicMaterialInstance` _decal))
      (bind _output_get (set `self.DecalMat` _returnvalue))
      (`DecalComponent.SetDecalMaterial` _decal _output_get))))

(event `CleanStain`
  (bind _toiletactor (`self.ToiletActor`))
  (bind _returnvalue (- (`self.Dirtiness`) (`self.CleaningStrength`)))
  (if (<= _returnvalue 0.2)
    (if (`self.HasAuthority` (`GameplayStatics.GetPlayerCharacter` 0))
      (if (`KismetSystemLibrary.IsValid` _toiletactor)
        (`KismetArrayLibrary.Array_RemoveItem` (`/Game/PlaneContent/Blueprints/Systems/PlaneActors/NeedActors/Toilet/BP_Toilet.StainInstances` _toiletactor) self)
        (`/Game/PlaneContent/Blueprints/Systems/PlaneActors/NeedActors/Toilet/BP_Toilet.CheckIsClean` _toiletactor))
      (`self.K2_DestroyActor`))
    (elif (`self.HasAuthority` (`GameplayStatics.GetPlayerCharacter` 0))
      (bind _output_get (set `self.Dirtiness` _returnvalue))
      (`MaterialInstanceDynamic.SetScalarParameterValue` (`self.DecalMat`) "Opacity" _output_get))))

(fn `OnRep_Dirtiness`
  (`MaterialInstanceDynamic.SetScalarParameterValue` (`self.DecalMat`) "Opacity" (`self.Dirtiness`)))

(fn `OnRep_Transform`
  (`self.K2_SetActorTransform` (`self.Transform`)))

(fn `UserConstructionScript`)