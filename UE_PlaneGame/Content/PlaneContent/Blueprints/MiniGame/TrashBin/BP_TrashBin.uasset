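; Trash bin for a minigame that swallows dropped Trash-tagged actors and yields a trash bag when full.
; A server-side overlap counts trash up to a maximum, flinging other or excess WorldItems upward in a random cone.
; The count moves and scales a fill plane, and a full bin enables a grab handle that spawns BP_TrashBag and empties it.
; RepNotifies sync fill visuals and handle collision to clients.
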(event `self.ReceiveBeginPlay`
  (bind _asbp_grab_handle (cast `/Game/PlaneContent/Blueprints/Systems/PlaneActors/GrabHandle/BP_GrabHandle` (`ChildActorComponent.ChildActor` (`self.BP_GrabHandle`))))
  (set `self.GrabHandle` _asbp_grab_handle)
  (add `GrabHandle.OnGrabbed` _asbp_grab_handle (`|CreateDelegate` :!event `OnGrabbed`))
  (add `GrabHandle.OnLetGo` _asbp_grab_handle (`|CreateDelegate` :!event `OnLetGo`))
  (`SceneComponent.SetVisibility` (`/Game/PlaneContent/Blueprints/Systems/PlaneActors/GrabHandle/BP_GrabHandle.Sphere` _asbp_grab_handle) false false)
  (`PrimitiveComponent.SetCollisionEnabled` (`/Game/PlaneContent/Blueprints/Systems/PlaneActors/GrabHandle/BP_GrabHandle.Sphere` (`self.GrabHandle`)) "NoCollision"))

(event `OnGrabbed`
  (params (Hand :type "PlayerHand Object Reference") (PlayerCharacter :type "PlanePlayerCharacter Object Reference"))
  (if (`self.IsInteractable`)
    (if (`self.HasAuthority` (`GameplayStatics.GetPlayerCharacter` 0))
      (`|SpawnActorFromClass` "/Game/PlaneContent/Blueprints/MiniGame/TrashBin/BP_TrashBag.BP_TrashBag_C" (`KismetMathLibrary.MakeTransform` (+ (* (`self.Vector`) 1.5) (`self.K2_GetActorLocation`))) "Undefined" "MultiplyWithRoot" null null)
      (set `self.CurrentTrashCount` 0)
      (`self.HandleTrashVisuals`))))

(event `OnLetGo`
  (params (Hand :type "PlayerHand Object Reference") (PlayerCharacter :type "PlanePlayerCharacter Object Reference")))

(event `self.Sphere.OnComponentBeginOverlap`
  (params (OverlappedComponent :type "PrimitiveComponent Object Reference") (OtherActor :type "Actor Object Reference") (OtherComp :type "PrimitiveComponent Object Reference") (OtherBodyIndex :type Integer) (bFromSweep :type Boolean) (SweepResult :type "HitResult Structure (by ref)"))
  (if (`self.HasAuthority` (`GameplayStatics.GetPlayerCharacter` 0))
    (if (`self.ActorHasTag` OtherActor "Trash")
      (if (< (`self.CurrentTrashCount`) (`self.MaxTrashItems`))
        (`self.K2_DestroyActor` OtherActor)
        (`/Engine/EditorBlueprintResources/StandardMacros.IncrementInt` (`self.CurrentTrashCount`)
          (:`  `
            (`self.HandleTrashVisuals`)))
        (else
          (`self.ThrowOutNonTrash` OtherActor :!label _label)))
      (else
        (goto _label)))))

(fn `HandleTrashVisuals`
  (bind _fillplane (`self.FillPlane`))
  (bind _sphere (`/Game/PlaneContent/Blueprints/Systems/PlaneActors/GrabHandle/BP_GrabHandle.Sphere` (`self.GrabHandle`)))
  (bind _returnvalue (+ (* (/ (- (`self.MaxScale`) (`self.MinScale`)) (`self.MaxTrashItems`)) (`self.CurrentTrashCount`)) (`self.MinScale`)))
  (`|ExecutionSequence`
    (:`then_0`
      (`SceneComponent.K2_SetRelativeTransform` (`self.FillPlane`) (`KismetMathLibrary.MakeTransform` (* (/ (`self.Vector`) (`self.MaxTrashItems`)) (`self.CurrentTrashCount`)) (struct) (`KismetMathLibrary.MakeVector` _returnvalue _returnvalue 1.0)) false false)
      (if (> (`self.CurrentTrashCount`) 0)
        (if (not (`SceneComponent.IsVisible` (`self.FillPlane`)))
          (`SceneComponent.SetVisibility` (`self.FillPlane`) true false))
        (elif (`SceneComponent.IsVisible` (`self.FillPlane`))
          (`SceneComponent.SetVisibility` (`self.FillPlane`) false false))))
    (:`then_1`
      (if (== (`self.CurrentTrashCount`) (`self.MaxTrashItems`))
        (`PrimitiveComponent.SetCollisionObjectType` _fillplane "ECC_WorldDynamic")
        (`PrimitiveComponent.SetCollisionEnabled` _fillplane "QueryAndPhysics")
        (else
          (`PrimitiveComponent.SetCollisionEnabled` (`self.FillPlane`) "NoCollision"))))
    (:`then_2`
      (if (`self.HasAuthority` (`GameplayStatics.GetPlayerCharacter` 0))
        (if (== (`self.CurrentTrashCount`) (`self.MaxTrashItems`))
          (if (not (`self.IsInteractable`))
            (set `self.IsInteractable` true)
            (`PrimitiveComponent.SetCollisionEnabled` _sphere "QueryAndPhysics"))
          (elif (`self.IsInteractable`)
            (set `self.IsInteractable` false)
            (`PrimitiveComponent.SetCollisionEnabled` _sphere "NoCollision")))))))

(fn `OnRep_CurrentTrashCount`
  (`self.HandleTrashVisuals`))

(fn `OnRep_IsInteractable`
  (bind _sphere (`/Game/PlaneContent/Blueprints/Systems/PlaneActors/GrabHandle/BP_GrabHandle.Sphere` (`self.GrabHandle`)))
  (if (`self.IsInteractable`)
    (`PrimitiveComponent.SetCollisionEnabled` _sphere "QueryAndPhysics")
    (else
      (`PrimitiveComponent.SetCollisionEnabled` _sphere "NoCollision"))))

(fn `ThrowOutNonTrash`
  (params (Object :type "Object Object Reference"))
  (bind _asworld_item (cast `WorldItem` Object))
  (`PrimitiveComponent.AddImpulse` (`self.GetComponentByClass` _asworld_item "/Script/Engine.StaticMeshComponent") (* (`KismetMathLibrary.RandomUnitVectorInConeInDegrees` (0.0 0.0 1.0) 20.0) 850.0) "None" false))

(fn `UserConstructionScript`)