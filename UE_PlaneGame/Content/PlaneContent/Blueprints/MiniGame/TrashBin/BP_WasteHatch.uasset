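; BP_WasteHatch is a trash bin hatch minigame actor that launches world items via three linked buttons.
; Holding Open or Close plays or reverses the front hatch timeline, stopping on release.
; Fire works only with the front shut, swinging the back hatch open, then impulsing overlapping WorldItems along the Arrow-to-actor direction, scaled by mass and Force.
; After audio and a delay, the back hatch closes, releasing the firing lock.
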(event `self.ReceiveBeginPlay`
  (`/Engine/EditorBlueprintResources/StandardMacros.IsValid` (`self.OpenButton`)
    (:`Is Valid`
      (add `WorldButton.OnButtonHold_Start` (`self.OpenButton`) (`|CreateDelegate` :!event `OnOpenHoldStart`))
      (add `WorldButton.OnButtonHold_End` (`self.OpenButton`) (`|CreateDelegate` :!event `OnOpenHoldEnd`))
      (`/Engine/EditorBlueprintResources/StandardMacros.IsValid` (`self.CloseButton`)
        (:`Is Valid`
          (add `WorldButton.OnButtonHold_Start` (`self.CloseButton`) (`|CreateDelegate` :!event `OnCloseHoldStart`))
          (add `WorldButton.OnButtonHold_End` (`self.CloseButton`) (`|CreateDelegate` :!event `OnCloseHoldEnd`))
          (`/Engine/EditorBlueprintResources/StandardMacros.IsValid` (`self.FireButton`)
            (:`Is Valid`
              (add `WorldButton.OnButtonPressed` (`self.FireButton`) (`|CreateDelegate` :!event `OnFireButtonPressed`)))))))))

(event `OnOpenHoldStart`
  (params (Player :type "PlanePlayerCharacter Object Reference"))
  (if (not (`self.isShootingTrash`))
    (bind (_direction _newtrack_0) (`Timeline|OpenHatch` :!label _label)
      (:`Update`
        (`SceneComponent.K2_SetRelativeRotation` (`self.HatchFront`) (`KismetMathLibrary.MakeRotator` (`KismetMathLibrary.Lerp` 0.0 (`self.OpenAngleFrontHatch`) _newtrack_0)) false false))
      (:`Finished`
        (if (`|EnumEquality` _direction "Forward")
          (`SceneComponent.K2_SetRelativeRotation` (`self.HatchFront`) (`KismetMathLibrary.MakeRotator` (`self.OpenAngleFrontHatch`)) false false)
          (else
            (`SceneComponent.K2_SetRelativeRotation` (`self.HatchFront`) (`KismetMathLibrary.MakeRotator` 0.0) false false)))))))

(event `OnOpenHoldEnd`
  (params (Player :type "PlanePlayerCharacter Object Reference"))
  (if (not (`self.isShootingTrash`)) :!label _label_2
    (goto _label :!via `Stop`)))

(event `OnCloseHoldEnd`
  (params (Player :type "PlanePlayerCharacter Object Reference"))
  (goto _label_2))

(event `OnCloseHoldStart`
  (params (Player :type "PlanePlayerCharacter Object Reference"))
  (if (not (`self.isShootingTrash`))
    (goto _label :!via `Reverse`)))

(event `OnFireButtonPressed`
  (params (Player :type "PlanePlayerCharacter Object Reference"))
  (bind _relativerotation_roll (`KismetMathLibrary.BreakRotator` (`SceneComponent.RelativeRotation` (`self.HatchFront`))))
  (if (and (== _relativerotation_roll 0.0) (not (`self.isShootingTrash`)))
    (set `self.isShootingTrash` true)
    (bind (_direction _newtrack_0) (`Timeline|BackHatch` :!via `PlayFromStart` :!label _label_3)
      (:`Update`
        (`SceneComponent.K2_SetRelativeRotation` (`self.HatchBack`) (`KismetMathLibrary.MakeRotator` (`KismetMathLibrary.Lerp` 0.0 90.0 _newtrack_0)) false false))
      (:`Finished`
        (if (`|EnumEquality` _direction "Forward")
          (for _array_element (`PrimitiveComponent.GetOverlappingActors` (`self.Box`) null)
            (bind _asworld_item (cast `WorldItem` _array_element))
            (bind _returnvalue (`self.GetComponentByClass` _asworld_item "/Script/Engine.StaticMeshComponent"))
            (`PrimitiveComponent.AddImpulse` _returnvalue (* (`KismetMathLibrary.Normal` (- (`self.K2_GetActorLocation`) (`SceneComponent.K2_GetComponentLocation` (`self.Arrow`)))) (* (`PrimitiveComponent.GetMass` _returnvalue) (`self.Force`))) "None" false))
          (`AudioComponent.Play` (`self.ShootAudio`) 0.0)
          (`KismetSystemLibrary.Delay` 1.0)
          (goto _label_3 :!via `Reverse`)
          (else
            (set `self.isShootingTrash` false)))))))

(fn `UserConstructionScript`)