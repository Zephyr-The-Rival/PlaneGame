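; Networked trash chute mini-game prop that swallows "Trash"-tagged actors and ejects other world items, or any arriving when full, with an upward impulse.
; An authority-checked count drives the fill plane's height and collision, and enables the grab handle when full; RepNotifies apply visuals, handle collision and physics.
; Grabbing enables physics and per-tick hand-driven impulses on the body; grabbing a full, sufficiently tilted chute instead spawns a trash bag and empties it.
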(event `self.ReceiveBeginPlay`
  (bind _asbp_grab_handle (cast `/Game/PlaneContent/Blueprints/Systems/PlaneActors/GrabHandle/BP_GrabHandle` (`ChildActorComponent.ChildActor` (`self.BP_GrabHandle`))))
  (set `self.GrabHandle` _asbp_grab_handle)
  (add `GrabHandle.OnGrabbed` _asbp_grab_handle (`|CreateDelegate` :!event `OnGrabbed`))
  (add `GrabHandle.OnLetGo` _asbp_grab_handle (`|CreateDelegate` :!event `OnLetGo`))
  (`SceneComponent.SetVisibility` (`/Game/PlaneContent/Blueprints/Systems/PlaneActors/GrabHandle/BP_GrabHandle.Sphere` _asbp_grab_handle) false false))

(event `OnGrabbed`
  (params (Hand :type "PlayerHand Object Reference") (PlayerCharacter :type "PlanePlayerCharacter Object Reference"))
  (bind (_vector_x _vector_y _vector_z) (`KismetMathLibrary.BreakVector` (`self.Vector`)))
  (bind (_returnvalue_x _returnvalue_y _returnvalue_z) (`KismetMathLibrary.BreakVector` (`SceneComponent.K2_GetComponentLocation` (`self.FillPlane`))))
  (bind _relativerotation_roll (`KismetMathLibrary.BreakRotator` (`SceneComponent.RelativeRotation` (`self.Body`))))
  (if (`self.IsInteractable`)
    (if (and (`self.HasAuthority` (`GameplayStatics.GetPlayerCharacter` 0)) (< _relativerotation_roll -35.0))
      (`|SpawnActorFromClass` "/Game/PlaneContent/Blueprints/MiniGame/TrashBin/BP_TrashBag.BP_TrashBag_C" (`KismetMathLibrary.MakeTransform` (`KismetMathLibrary.MakeVector` _returnvalue_x _returnvalue_y (+ (* _vector_z 1.5) _returnvalue_z))) "Undefined" "MultiplyWithRoot" null null)
      (set `self.CurrentTrashCount` 0)
      (`self.HandleTrashVisuals`)
      (else
        (set `self.SimulatePhysics` true :!label _label)
        (`KismetArrayLibrary.Array_Add` (`self.Hands`) Hand)
        (`KismetArrayLibrary.Array_Add` (`self.Player`) PlayerCharacter)
        (set `self.ApplyForce` true)))
    (else
      (goto _label))))

(event `self.ReceiveTick`
  (params (DeltaSeconds :type "Float (single-precision)"))
  (`self.ApplyForceToPlayer`))

(event `ApplyForceToPlayer`
  (bind _returnvalue (`SceneComponent.K2_GetComponentLocation` (`self.BP_GrabHandle`)))
  (bind _returnvalue_2 (* (`KismetMathLibrary.Normal` (`self.ForceVector`)) (`self.Force`)))
  (if (`self.ApplyForce`)
    (set `self.ForceVector` (0.0 0.0 0.0))
    (for (_ _array_index) (`self.Hands`)
      (set `self.ForceVector` (`KismetMathLibrary.ProjectVectorOnToPlane` (+ (`self.ForceVector`) (- (`self.K2_GetActorLocation` (`PlanePlayerCharacter.MyPlayerHand` (`|GetArrayItem` (`self.Player`) _array_index))) (`SceneComponent.K2_GetComponentLocation` (`self.BP_GrabHandle`)))) (`SceneComponent.GetForwardVector` (`self.Arrow`)))))
    (`PrimitiveComponent.AddImpulseAtLocation` (`self.Body`) _returnvalue_2 _returnvalue "None")
    (`KismetSystemLibrary.DrawDebugLine` _returnvalue (+ _returnvalue _returnvalue_2) (struct :`G` 0.295438 :`B` 1.0 :`A` 1.0) 0.1 1.0)))

(event `OnLetGo`
  (params (Hand :type "PlayerHand Object Reference") (PlayerCharacter :type "PlanePlayerCharacter Object Reference"))
  (`|ExecutionSequence`
    (:`then_0`
      (`KismetArrayLibrary.Array_RemoveItem` (`self.Hands`) Hand)
      (`KismetArrayLibrary.Array_RemoveItem` (`self.Player`) PlayerCharacter))
    (:`then_1`
      (if (`KismetArrayLibrary.Array_IsEmpty` (`self.Hands`))
        (set `self.SimulatePhysics` false)
        (set `self.ApplyForce` false)))))

(event `self.Box.OnComponentBeginOverlap`
  (params (OverlappedComponent :type "PrimitiveComponent Object Reference") (OtherActor :type "Actor Object Reference") (OtherComp :type "PrimitiveComponent Object Reference") (OtherBodyIndex :type Integer) (bFromSweep :type Boolean) (SweepResult :type "HitResult Structure (by ref)"))
  (if (`self.HasAuthority` (`GameplayStatics.GetPlayerCharacter` 0))
    (if (`self.ActorHasTag` OtherActor "Trash")
      (if (< (`self.CurrentTrashCount`) (`self.MaxTrashItems`))
        (`self.K2_DestroyActor` OtherActor)
        (`/Engine/EditorBlueprintResources/StandardMacros.IncrementInt` (`self.CurrentTrashCount`)
          (:`  `
            (`self.HandleTrashVisuals`)))
        (else
          (`self.ThrowOutNonTrash` OtherActor :!label _label_2)))
      (else
        (goto _label_2)))))

(fn `HandleTrashVisuals`
  (bind _fillplane (`self.FillPlane`))
  (bind (_relativelocation_x _relativelocation_y) (`KismetMathLibrary.BreakVector` (`SceneComponent.RelativeLocation` (`self.FillPlane`))))
  (bind (_returnvalue_x _returnvalue_y _returnvalue_z) (`KismetMathLibrary.BreakVector` (* (/ (`self.Vector`) (`self.MaxTrashItems`)) (`self.CurrentTrashCount`))))
  (`|ExecutionSequence`
    (:`then_0`
      (`SceneComponent.K2_SetRelativeTransform` (`self.FillPlane`) (`KismetMathLibrary.MakeTransform` (`KismetMathLibrary.MakeVector` _relativelocation_x _relativelocation_y _returnvalue_z) (struct) (1.0 1.0 1.0)) false false)
      (if (> (`self.CurrentTrashCount`) 0)
        (if (not (`SceneComponent.IsVisible` (`self.FillPlane`)))
          (`SceneComponent.SetVisibility` (`self.FillPlane`) true false))
        (elif (`SceneComponent.IsVisible` (`self.FillPlane`))
          (`SceneComponent.SetVisibility` (`self.FillPlane`) false false))))
    (:`then_1`
      (if (== (`self.CurrentTrashCount`) (`self.MaxTrashItems`))
        (`PrimitiveComponent.SetCollisionObjectType` _fillplane "ECC_WorldDynamic")
        (`PrimitiveComponent.SetCollisionEnabled` _fillplane "QueryAndPhysics")
        (else
          (`PrimitiveComponent.SetCollisionEnabled` (`self.FillPlane`) "NoCollision"))))
    (:`then_2`
      (if (`self.HasAuthority` (`GameplayStatics.GetPlayerCharacter` 0))
        (if (== (`self.CurrentTrashCount`) (`self.MaxTrashItems`))
          (if (not (`self.IsInteractable`))
            (set `self.IsInteractable` true))
          (elif (`self.IsInteractable`)
            (set `self.IsInteractable` false)))))))

(fn `OnRep_CurrentTrashCount`
  (`self.HandleTrashVisuals`))

(fn `OnRep_IsInteractable`
  (bind _sphere (`/Game/PlaneContent/Blueprints/Systems/PlaneActors/GrabHandle/BP_GrabHandle.Sphere` (`self.GrabHandle`)))
  (if (`self.IsInteractable`)
    (`PrimitiveComponent.SetCollisionEnabled` _sphere "QueryAndPhysics")
    (else
      (`PrimitiveComponent.SetCollisionEnabled` _sphere "NoCollision"))))

(fn `OnRep_SimulatePhysics`
  (`PrimitiveComponent.SetSimulatePhysics` (`self.Body`) (`self.SimulatePhysics`)))

(fn `ThrowOutNonTrash`
  (params (Object :type "Object Object Reference"))
  (bind _asworld_item (cast `WorldItem` Object))
  (`PrimitiveComponent.AddImpulse` (`self.GetComponentByClass` _asworld_item "/Script/Engine.StaticMeshComponent") (* (`KismetMathLibrary.RandomUnitVectorInConeInDegrees` (`SceneComponent.GetUpVector` (`self.FillPlane`)) 2.0) 1300.0) "None" false))

(fn `UserConstructionScript`)