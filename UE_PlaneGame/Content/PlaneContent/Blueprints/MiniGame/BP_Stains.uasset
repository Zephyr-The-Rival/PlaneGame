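; BP_Stains is a cleanable decal stain for a lavatory cleaning minigame.
; Each CleanStain call lowers Dirtiness and decal opacity; near the threshold, the stain leaves its lavatory's list, triggers CheckIsClean and destroys itself.
; DrawBrush paints a brush material at a normalized location into a per-stain render target fed to the decal's dynamic material.
; The construction script scales decal and plane from StainsTransfrom, swapping X and Z for the decal.
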(event `self.ReceiveBeginPlay`
  (bind _decal (`self.Decal`))
  (`|ExecutionSequence`
    (:`then_0`
      (bind _returnvalue (`DecalComponent.CreateDynamicMaterialInstance` _decal))
      (bind _returnvalue_2 (`KismetRenderingLibrary.CreateRenderTarget2D` 1024 1024))
      (bind _output_get (set `self.DecalMat` _returnvalue))
      (`DecalComponent.SetDecalMaterial` _decal _output_get)
      (bind _output_get_2 (set `self.RenderTarget` _returnvalue_2))
      (`MaterialInstanceDynamic.SetTextureParameterValue` _returnvalue "RenderTarget" _output_get_2))
    (:`then_1`
      (bind _returnvalue_3 (`KismetMaterialLibrary.CreateDynamicMaterialInstance` "/Game/PlaneContent/Assets/MiniGame/Toilet/mat/M_Brush.M_Brush"))
      (set `self.BrushMat` _returnvalue_3))))

(event `CleanStain`
  (bind _lavatoryins (`self.LavatoryIns`))
  (bind _returnvalue (- (`self.Dirtiness`) (`self.CleaningStrength`)))
  (if (<= _returnvalue 0.2)
    (if (`KismetSystemLibrary.IsValid` _lavatoryins)
      (`KismetArrayLibrary.Array_RemoveItem` (`/Game/PlaneContent/Blueprints/MiniGame/BP_Lavatory.Sains instances` _lavatoryins) self)
      (`/Game/PlaneContent/Blueprints/MiniGame/BP_Lavatory.CheckIsClean` _lavatoryins))
    (`self.K2_DestroyActor`)
    (else
      (bind _output_get (set `self.Dirtiness` _returnvalue))
      (`MaterialInstanceDynamic.SetScalarParameterValue` (`self.DecalMat`) "Opacity" _output_get))))

(fn `DrawBrush`
  (params (BrushTexture :type "Texture2D Object Reference") (BrushSize :type "Float (double-precision)") (DrawLocation :type "Vector2D Structure"))
  (bind _brushsize (`local.BrushSize`))
  (`|ExecutionSequence`
    (:`then_0`
      (`MaterialInstanceDynamic.SetTextureParameterValue` (`self.BrushMat`) "Brushtexture" BrushTexture))
    (:`then_1`
      (bind (_canvas _size _context) (`KismetRenderingLibrary.BeginDrawCanvasToRenderTarget` (`self.RenderTarget`)))
      (`Canvas.K2_DrawMaterial` _canvas (`self.BrushMat`) (- (* _size (`local.DrawLocation`)) (/ _brushsize 2.0)) (`KismetMathLibrary.MakeVector2D` _brushsize _brushsize) (0.0 0.0) (1.0 1.0) 0.0 (0.5 0.5))
      (`KismetRenderingLibrary.EndDrawCanvasToRenderTarget` _context))))

(fn `UserConstructionScript`
  (bind (_stainstransfrom_x _stainstransfrom_y _stainstransfrom_z) (`KismetMathLibrary.BreakVector` (`self.StainsTransfrom`)))
  (`|ExecutionSequence`
    (:`then_0`
      (`SceneComponent.SetRelativeScale3D` (`self.Decal`) (`KismetMathLibrary.MakeVector` _stainstransfrom_z _stainstransfrom_y _stainstransfrom_x)))
    (:`then_1`
      (`SceneComponent.SetRelativeScale3D` (`self.Plane`) (`KismetMathLibrary.MakeVector` _stainstransfrom_x _stainstransfrom_y _stainstransfrom_z)))))