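; Coffee machine for a minigame that snaps in a released coffee jug and fills it while running.
; A capsule overlap detects the jug, with Tick polling until the player's hand lets go before teleporting it to an offset.
; A world button, spawned and bound with authority, runs the machine for a fixed delay if a jug is present.
; The IsMaschineOn RepNotify toggles audio and Niagara effects, while Tick calls FillJug.
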(event `self.ReceiveBeginPlay`
  (`self.InitButton`))

(event `OnButtonPressed`
  (params (Player :type "PlanePlayerCharacter Object Reference"))
  (if (`self.HasAuthority` (`GameplayStatics.GetPlayerCharacter` 0))
    (`/Engine/EditorBlueprintResources/StandardMacros.IsValid` (`self.CoffeeJug`)
      (:`Is Valid`
        (if (not (`self.IsMaschineOn`))
          (set `self.IsMaschineOn` true)
          (`KismetSystemLibrary.Delay` 10.0)
          (set `self.IsMaschineOn` false))))))

(event `self.Capsule.OnComponentBeginOverlap`
  (params (OverlappedComponent :type "PrimitiveComponent Object Reference") (OtherActor :type "Actor Object Reference") (OtherComp :type "PrimitiveComponent Object Reference") (OtherBodyIndex :type Integer) (bFromSweep :type Boolean) (SweepResult :type "HitResult Structure (by ref)"))
  (`self.PlacingJugIsValid` OtherActor)
  (`self.IsPlayerHoldingJug` OtherActor
    (:`Holding`
      (set `self.CheckForPlayerLetGoJug` true))
    (:`Not Holding`
      (`self.PlaceJugInMaschine` OtherActor))))

(event `self.ReceiveTick`
  (params (DeltaSeconds :type "Float (single-precision)"))
  (if (and (`self.CheckForPlayerLetGoJug`) (not (`self.JugInMaschine`)))
    (for _array_element (`PrimitiveComponent.GetOverlappingActors` (`self.Capsule`) "/Game/PlaneContent/Blueprints/MiniGame/Coffee/BP_CoffeeJug.BP_CoffeeJug_C")
      (`self.IsPlayerHoldingJug` _array_element
        (:`Not Holding`
          (`self.PlaceJugInMaschine` _array_element)
          (break))))
    (elif (`self.JugInMaschine`)
      (`|ExecutionSequence`
        (:`then_0`
          (`/Engine/EditorBlueprintResources/StandardMacros.IsValid` (`self.CoffeeJug`)
            (:`Is Valid`
              (if (`self.IsMaschineOn`)
                (`/Game/PlaneContent/Blueprints/MiniGame/Coffee/BP_CoffeeJug.FillJug` (`self.CoffeeJug`))))))
        (:`then_1`
          (if (`KismetArrayLibrary.Array_IsEmpty` (`PrimitiveComponent.GetOverlappingActors` (`self.Capsule`) "/Game/PlaneContent/Blueprints/MiniGame/Coffee/BP_CoffeeJug.BP_CoffeeJug_C")) :!label _label
            (set `self.JugInMaschine` false)
            (set `self.CheckForPlayerLetGoJug` false)
            (set `self.CoffeeJug` null)))))))

(event `self.Capsule.OnComponentEndOverlap`
  (params (OverlappedComponent :type "PrimitiveComponent Object Reference") (OtherActor :type "Actor Object Reference") (OtherComp :type "PrimitiveComponent Object Reference") (OtherBodyIndex :type Integer))
  (goto _label))

(fn `InitButton`
  (bind (_buttonspawnlocation_location _buttonspawnlocation_rotation _buttonspawnlocation_scale) (`KismetMathLibrary.BreakTransform` (`self.ButtonSpawnLocation`)))
  (if (`self.HasAuthority` (`GameplayStatics.GetPlayerCharacter` 0))
    (bind _returnvalue (`|SpawnActorFromClass` "/Game/PlaneContent/Blueprints/Systems/Button/BP_WorldButton.BP_WorldButton_C" (`KismetMathLibrary.MakeTransform` (+ _buttonspawnlocation_location (`self.K2_GetActorLocation`)) _buttonspawnlocation_rotation _buttonspawnlocation_scale) "Undefined" "MultiplyWithRoot" null null))
    (set `self.Button` _returnvalue)
    (add `WorldButton.OnButtonPressed` (`self.Button`) (`|CreateDelegate` :!event `OnButtonPressed`))))

(fn `OnRep_IsMaschineOn`
  (bind _ismaschineon (`self.IsMaschineOn`))
  (`KismetSystemLibrary.PrintString` (`KismetStringLibrary.Conv_BoolToString` _ismaschineon))
  (if _ismaschineon
    (`AudioComponent.Play` (`self.Audio`) 0.0)
    (`ActorComponent.Activate` (`self.NS_CoffeeMachine`) false)
    (else
      (`AudioComponent.Stop` (`self.Audio`))
      (`ActorComponent.Deactivate` (`self.NS_CoffeeMachine`)))))

(fn `PlaceJugInMaschine`
  (params (Actor :type "Actor Object Reference"))
  (bind _offsetjugtransform_location (`KismetMathLibrary.BreakTransform` (`self.OffsetJugTransform`)))
  (bind (_returnvalue_roll _returnvalue_pitch _returnvalue_yaw) (`KismetMathLibrary.BreakRotator` (`SceneComponent.K2_GetComponentRotation` (`self.DefaultSceneRoot`))))
  (bind _asbp_coffee_jug (cast `/Game/PlaneContent/Blueprints/MiniGame/Coffee/BP_CoffeeJug` Actor))
  (`self.K2_SetActorTransform` _asbp_coffee_jug (`KismetMathLibrary.MakeTransform` (+ (`KismetMathLibrary.GreaterGreater_VectorRotator` _offsetjugtransform_location (`SceneComponent.K2_GetComponentRotation` (`self.DefaultSceneRoot`))) (`self.K2_GetActorLocation`)) (`KismetMathLibrary.MakeRotator` _returnvalue_roll _returnvalue_pitch (+ _returnvalue_yaw (.yaw (.rotation (`self.OffsetJugTransform`)))))) false true)
  (set `self.JugInMaschine` true)
  (set `self.CoffeeJug` _asbp_coffee_jug))

(fn `UserConstructionScript`)