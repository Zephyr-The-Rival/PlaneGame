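; Coffee jug for the coffee minigame, which can be filled over time and pours coffee into cups.
; Its tank component receives the spill Niagara system and drives a percentage text that hides when empty.
; FillJug adds frame-rate-independent amounts to the tank.
; HandleCoffeeParticles takes particle data, sphere-overlaps at each position and slightly fills the nearest overlapping BP_Cup's tank, so pouring follows the particles.
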(event `self.ReceiveBeginPlay`
  (set `/Game/PlaneContent/Blueprints/Components/Tank/AC_Tank.NS Coffee Spilling` (`self.NS_CoffeeSpilling`) (`self.AC_Tank`))
  (add `/Game/PlaneContent/Blueprints/Components/Tank/AC_Tank.OnTankChanged` (`self.AC_Tank`) (`|CreateDelegate` :!event `OnTankChanged`))
  (add `/Game/PlaneContent/Blueprints/Components/Tank/AC_Tank.OnTankEmpty` (`self.AC_Tank`) (`|CreateDelegate` :!event `OnTankEmpty`))
  (add `/Game/PlaneContent/Blueprints/Components/Tank/AC_Tank.OnTankFull` (`self.AC_Tank`) (`|CreateDelegate` :!event `OnTankFull`)))

(event `OnTankChanged`
  (params (NewTankLevel :type "Float (double-precision)"))
  (`TextRenderComponent.K2_SetText` (`self.TextRender`) (`KismetSystemLibrary.MakeLiteralText` (`KismetTextLibrary.Conv_DoubleToText` (* NewTankLevel 100.0) "HalfToEven" false true 1 324 0 0)))
  (if (not (`SceneComponent.bVisible` (`self.TextRender`)))
    (`SceneComponent.SetVisibility` (`self.TextRender`) true false)))

(event `OnTankEmpty`
  (`SceneComponent.SetVisibility` (`self.TextRender`) false false))

(event `OnTankFull`)

(fn `FillJug`
  (`/Game/PlaneContent/Blueprints/Components/Tank/AC_Tank.FillTank` (`self.AC_Tank`) (* (`self.FillSpeed`) (`GameplayStatics.GetWorldDeltaSeconds`))))

(fn `HandleCoffeeParticles`
  (params (Array :type "Array of BasicParticleData Structure"))
  (locals (ShortestDistance :type "Float (double-precision)") (Cup :type "/Game/PlaneContent/Blueprints/Items/BP_Cup Object Reference"))
  (bind _cup (`local.Cup`))
  (for _array_element Array
    (`|ExecutionSequence`
      (:`then_0`
        (bind _position (break `BasicParticleData` _array_element))
        (bind (_outactors _returnvalue) (`KismetSystemLibrary.SphereOverlapActors` _position 8.0 (`|MakeArray` "ObjectTypeQuery2" :!type "EObjectTypeQuery Enum")))
        (if _returnvalue
          (set `local.ShortestDistance` 10000000000.0)
          (set `local.Cup` null)
          (for _array_element_2 _outactors
            (bind _asbp_cup (cast `/Game/PlaneContent/Blueprints/Items/BP_Cup` _array_element_2))
            (bind _returnvalue_2 (`KismetMathLibrary.Vector_DistanceSquared` (`self.K2_GetActorLocation` _asbp_cup) _position))
            (if (< _returnvalue_2 (`local.ShortestDistance`))
              (set `local.ShortestDistance` _returnvalue_2)
              (set `local.Cup` _asbp_cup)))
          (`/Engine/EditorBlueprintResources/StandardMacros.IsValid` _cup
            (:`Is Valid`
              (`/Game/PlaneContent/Blueprints/Components/Tank/AC_Tank.FillTank` (`/Game/PlaneContent/Blueprints/Items/BP_Cup.AC_Tank` _cup) 0.01))))))))

(fn `UserConstructionScript`)