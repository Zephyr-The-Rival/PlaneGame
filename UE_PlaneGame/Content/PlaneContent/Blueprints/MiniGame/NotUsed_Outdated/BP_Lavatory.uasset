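; BP_Lavatory is an outdated lavatory actor for a toilet-cleaning minigame, kept in the NotUsed_Outdated folder.
; GeneratingStains spawns BP_Stains at saved transforms offset by the actor's location, stores the instances and sets IsDirty.
; CheckIsClean prints either a clean message or the remaining stain count from that array, without clearing IsDirty.
; An internal note flags a missing reference after a switch to BP_Toilet for NPC use.
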(event `Generating Stains`
  (for _array_element (`self.Saved stans transfrom`)
    ; Ref Missing. Zhu i changed this to the BP_Toilet Actor for npc purposes
    (bind _returnvalue (`|SpawnActorFromClass` "/Game/PlaneContent/Blueprints/MiniGame/Cleaning/BP_Stains.BP_Stains_C" (`KismetMathLibrary.MakeTransform` (+ (.location _array_element) (`self.K2_GetActorLocation`)) (.rotation _array_element) (.scale _array_element)) "Undefined" "MultiplyWithRoot" null null null))
    (`KismetArrayLibrary.Array_Add` (`self.Sains instances`) _returnvalue)
    (`KismetSystemLibrary.PrintString` "Toilet is fucked" true true (struct :`R` 1.0 :`G` 0.086621 :`B` 0.056774 :`A` 1.0) 5.0 "1"))
  (set `self.bIsDirty` true))

(event `CheckIsClean`
  (bind _sains_instances (`self.Sains instances`))
  (if (`KismetArrayLibrary.Array_IsEmpty` _sains_instances)
    (`KismetSystemLibrary.PrintString` "Toilet is clean" true true (struct :`G` 1.0 :`B` 0.247149 :`A` 1.0) 5.0 "1")
    (else
      (`KismetSystemLibrary.PrintString` (`KismetStringLibrary.Concat_StrStr` "Stans left: " (`KismetStringLibrary.Conv_IntToString` (`KismetArrayLibrary.Array_Length` _sains_instances))) true true (struct :`R` 1.0 :`G` 0.736817 :`B` 0.371494 :`A` 1.0) 2.0 "1"))))

(fn `UserConstructionScript`)